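; BP_Torch is a torch structure in the building system that can be lit or put out through interaction.
; The interact event toggles IsTorchLit, whose RepNotify shows or hides the fire component to match.
; On destruction, a one-time guard calls the parent destroy handler, then removes the actor after a short delay.
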(event EventInteractEvent
  (params (CharRef :type BP%20First%20Person%20Man%20Object%20Reference))
  (if (Variables|Default|GetIsTorchLit?)
    (Variables|Default|SetIsTorchLit? false)
    (else
      (Variables|Default|SetIsTorchLit? true))))

(event EventStructureDestroyEvent
  (params (DemolishedOrDestroyed? :type Boolean) (PlayerName :type Text))
  (if (not (Variables|Default|GetIsDestroyed?))
    (Variables|Default|SetIsDestroyed? true)
    (|CallParentFunction DemolishedOrDestroyed? PlayerName)
    (Utilities|FlowControl|Delay 3.0)
    (Actor|DestroyActor)))

(fn ConstructionScript
  (|CallParentFunction))

(fn OnRepIsTorchLit?
  (Rendering|SetVisibility (Variables|Default|GetP_TorchFire) (Variables|Default|GetIsTorchLit?) false))