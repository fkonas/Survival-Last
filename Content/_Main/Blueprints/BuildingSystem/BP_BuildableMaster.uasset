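; Base actor for buildable structures in the survival building system, handling damage, demolition, ownership and an info widget.
; Damage applies only when the causer's interface lists this structure's tier, and destruction multicasts a swap to a physics-simulated destructible mesh with a spawned force actor.
; Tribe-owned structures log their destruction through the game state.
; A server-checked overlap sphere shows players health and owner, enabling options for the owning player or tribe.
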(event OnComponentBeginOverlap(TextInfoSphere)
  (params (OverlappedComponent :type Primitive%20Component%20Object%20Reference) (OtherActor :type Actor%20Object%20Reference) (OtherComp :type Primitive%20Component%20Object%20Reference) (OtherBodyIndex :type Integer) (bFromSweep :type Boolean) (SweepResult :type Hit%20Result%20Structure%20%28by%20ref%29))
  ;[0 0 0] Show Or Hide Buildable Info Widget
  (Networking|SwitchHasAuthority
    (:Authority
      (if (Actor|ActorHasTag OtherActor "player")
        (bind _survivalcharref (Class|BPISurvivalCharacter|GetSurvivalCharRef(Message) OtherActor))
        (if (Variables|Default|GetPlayerOrTribeOwned?)
          (Default|ShoworHideInfo _survivalcharref self "Visible" (Variables|Default|GetShow%20Interact%20Text?) (Variables|Default|GetStructure%20Name) (Variables|Default|GetCurrentHP) (Variables|Default|GetMaxHP) (Variables|Default|GetOwner%20Name) (Utilities|Enum|Equal(Enum) (Class|AdvancedSessionsLibrary|UniqueNetIdtoString (Class|AdvancedSessionsLibrary|GetUniqueNetIDfromPlayerState (Variables|/Script/Engine.Pawn|GetPlayerState _survivalcharref))) (Variables|Default|GetOwnerNetID)))
          (else
            (bind _tribeid (Class|BPISurvivalPlayerState|GetTribeID(Message) (Variables|/Script/Engine.Pawn|GetPlayerState _survivalcharref)))
            (Default|ShoworHideInfo _survivalcharref self "Visible" (Variables|Default|GetShow%20Interact%20Text?) (Variables|Default|GetStructure%20Name) (Variables|Default|GetCurrentHP) (Variables|Default|GetMaxHP) (Variables|Default|GetOwner%20Name) (Utilities|Enum|Equal(Enum) _tribeid (Variables|Default|GetTribeID)))))))))

(event OnComponentEndOverlap(TextInfoSphere)
  (params (OverlappedComponent :type Primitive%20Component%20Object%20Reference) (OtherActor :type Actor%20Object%20Reference) (OtherComp :type Primitive%20Component%20Object%20Reference) (OtherBodyIndex :type Integer))
  ;[0 0 0] Show Or Hide Buildable Info Widget
  (Networking|SwitchHasAuthority
    (:Authority
      (if (Actor|ActorHasTag OtherActor "player")
        (bind _survivalcharref (Class|BPISurvivalCharacter|GetSurvivalCharRef(Message) OtherActor))
        (Default|ShoworHideInfo _survivalcharref self "Hidden" false "" 0.0 0.0 "" false)))))

(event Custom|MulticastDestruction
  (bind _staticmesh (Variables|Default|GetStaticMesh))
  (bind _destructablemesh (Variables|Default|GetDestructableMesh))
  (Collision|SetCollisionEnabled _staticmesh "NoCollision")
  (Rendering|SetVisibility _staticmesh false false)
  (Rendering|SetVisibility _destructablemesh true false)
  (Physics|SetSimulatePhysics _destructablemesh true)
  (Game|SpawnActorfromClass "/Game/_Main/Blueprints/HarvistingSystem/Destructable/BP_DestructionForce.BP_DestructionForce_C" (Math|Transform|MakeTransform (Transformation|GetActorLocation) "0, 0, 0" "1.000000,1.000000,1.000000") "Undefined" "MultiplyWithRoot" 0 0))

(event Custom|ShowText
  (params (IsVisible :type ESlateVisibility%20Enum :default "Visible") (ShowInteractText? :type Boolean) (StructureName :type Text) (CurentHP :type Float%20%28double-precision%29) (MaxHP :type Float%20%28double-precision%29) (OwnerName :type Text) (ShowOptionsText? :type Boolean))
  ;[0 0 0] Show Or Hide Buildable Info Widget
  (bind _asw_interact_text (Utilities|Casting|CastToW_InteractText (UserInterface|GetUserWidgetObject (Variables|Default|GetBuildableInfoWidget))))
  (Default|SetInteractShoworHide _asw_interact_text IsVisible ShowInteractText? StructureName CurentHP MaxHP OwnerName ShowOptionsText?))

(event Custom|PostDestructionToLog
  (params (DemolishedOrDestroyed? :type Boolean) (PlayerName :type Text))
  ;[1 1 1] Post Event to Tribe Log
  (Utilities|FlowControl|DoOnce false
    (:Completed
      (bind _gamestateref (Class|BPISurvivalGameState|GetGameStateRef(Message) (Game|GetGameState)))
      (Default|AddTribeLogEvent _gamestateref (Variables|Default|GetTribeID) (Utilities|Struct|MakeS_TribeLogEntry (Utilities|Text|ToText(Float) (Utilities|Time|GetGameTimeinSeconds) "HalfToEven") "1" (select DemolishedOrDestroyed? (Utilities|Text|FormatText "{playername} Has Demolished {StructureName}!" PlayerName (Variables|Default|GetStructure%20Name)) (Utilities|Text|FormatText "Your {StructureName} Was Destroyed!" (Variables|Default|GetStructure%20Name))) "NewEnumerator0")))))

(event Game|Damage|EventAnyDamage
  (params (Damage :type Float%20%28single-precision%29) (DamageType :type Damage%20Type%20Object%20Reference) (InstigatedBy :type Controller%20Object%20Reference) (DamageCauser :type Actor%20Object%20Reference))
  ;[0 0 0] Apply Damage To Structure
  (if (Utilities|DoesObjectImplementInterface DamageCauser "/Game/_Main/Blueprints/Interfaces/BPI_StructureDamage.BPI_StructureDamage_C")
    (bind _canapplydamage_ (CallFunction|CanDamageStructure? DamageCauser))
    (if _canapplydamage_
      (if (Variables|Default|GetCanDestroy?)
        (bind _output_get (Variables|Default|SetCurrentHP (- (Variables|Default|GetCurrentHP) Damage)))
        (Development|PrintString (Utilities|String|ToString(Float) _output_get))
        (if (<= (Variables|Default|GetCurrentHP) 0.0)
          (CallFunction|StructureDestroyEvent false))))))

(event EventStructureDestroyEvent
  (params (DemolishedOrDestroyed? :type Boolean) (PlayerName :type Text))
  (CallFunction|MulticastDestruction)
  (if (not (Variables|Default|GetPlayerOrTribeOwned?))
    (CallFunction|PostDestructiontoLog DemolishedOrDestroyed? PlayerName)))

(event EventDemolishStructure
  (params (PlayerName :type Text))
  (if (Variables|Default|GetCanDestroy?)
    (CallFunction|StructureDestroyEvent true PlayerName)))

(fn ConstructionScript)

(fn CanDamageStructure?
  (params (Instigator :type Object%20Object%20Reference))
  (Utilities|IsValid Instigator
    (:Is%20Valid
      (bind _damagetiers (Class|BPIStructureDamage|GetCanDamage(Message) Instigator))
      (bind _array_element (Utilities|Array|ForEachLoopwithBreak (Utilities|Struct|BreakS_DamageTiers _damagetiers) :!label _label)
        (:LoopBody
          (if (Utilities|Enum|Equal(Enum) _array_element (Variables|Default|GetStructureTier))
            (LocalVariables|SetCanDamage? true)
            (goto _label Break)))
        (:Completed
          (return (LocalVariables|GetCanDamage?)))))))

(fn CanPlaceCeiling?
  (return false))

(fn GetBuildMasterRef
  (return self))

(fn GetOwnerInfo
  (return (not (Variables|Default|GetPlayerOrTribeOwned?)) (Variables|Default|GetTribeID) (Variables|Default|GetOwnerNetID)))

(fn ReturnBoxes
  (return 0))