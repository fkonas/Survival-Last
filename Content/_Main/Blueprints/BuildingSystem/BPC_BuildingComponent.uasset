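; Building component on the survival character that previews structures from DT_Structures and spawns them on the server.
; A looping client camera trace moves a green/red preview, snapping it to boxes on the hit actor.
; Placement rules combine box overlap, ground-support, ceiling and foundation-tag checks, toggled by each buildable's info.
; On spawn, the server checks the hotbar item, repeats placement checks from client camera data, removes the item and spawns at the client-sent transform.
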(event Custom|LaunchBuildMode
  (params (StructureID :type Integer))
  ;[0 0 0] Build Mode On Client
  (if (Variables|Default|GetIsBuildModeEnabled?)
    (CallFunction|StopBuildLoop)
    (else
      (Variables|Default|SetIsBuildModeEnabled? true)
      (CallFunction|BuildModeClient StructureID))))

(event Custom|BuildLoop
  (bind _buildpreview (Variables|Default|GetBuildPreview))
  ;[0 0 0] Build Mode On Client
  (if (Variables|Default|GetIsBuildModeEnabled?)
    (Utilities|FlowControl|Delay 0.01)
    (CallFunction|BuildModeClient)
    (else
      (Variables|Default|SetIsBuildModeEnabled? false)
      (Utilities|IsValid _buildpreview
        (:Is%20Valid
          (Actor|DestroyActor _buildpreview))))))

(event Custom|StopBuildLoop
  (bind _buildpreview (Variables|Default|GetBuildPreview))
  ;[0 0 0] Build Mode On Client
  (Variables|Default|SetIsBuildModeEnabled? false)
  (Utilities|IsValid _buildpreview
    (:Is%20Valid
      (Actor|DestroyActor _buildpreview))))

(event Custom|SpawnBuildOnServer
  (params (Transform :type Transform) (ClientCameraVector :type Vector) (ClientCameraRotation :type Rotator))
  ;[0 0 0] Spawn Buildable On Server Event and Checks
  (Networking|SwitchHasAuthority
    (:Authority
      (Variables|Default|SetBuildTransform Transform)
      (bind _survivalcharref (Class|BPISurvivalCharacter|GetSurvivalCharRef(Message) (Components|GetOwner)))
      (bind _cancraft_ (Default|ContainsItems (Variables|/Game/_Main/Blueprints/Character/BP_FirstPersonMan.BP_FirstPersonMan_C|GetBPC_PlayerHotBar _survivalcharref) (Utilities|Array|MakeArray (Utilities|Struct|MakeS_ItemStruct (Variables|/Game/_Main/Blueprints/Character/BP_FirstPersonMan.BP_FirstPersonMan_C|GetStructureID _survivalcharref) 1))))
      (if _cancraft_
        (bind _canbuild_ (CallFunction|BuildPlacementCheck (Variables|/Game/_Main/Blueprints/Character/BP_FirstPersonMan.BP_FirstPersonMan_C|GetStructureID _survivalcharref) ClientCameraVector ClientCameraRotation))
        (if _canbuild_
          (bind _removed_ (Default|RemoveQuantity (Variables|/Game/_Main/Blueprints/Character/BP_FirstPersonMan.BP_FirstPersonMan_C|GetBPC_PlayerHotBar _survivalcharref) (Variables|/Game/_Main/Blueprints/Character/BP_FirstPersonMan.BP_FirstPersonMan_C|GetHotbarIndex _survivalcharref) 1))
          (if _removed_
            _
            (else
              _))
          (CallFunction|SpawnBuildable Transform (Variables|/Game/_Main/Blueprints/Character/BP_FirstPersonMan.BP_FirstPersonMan_C|GetStructureID _survivalcharref))
          (else
            (bind _buildpreview (Variables|Default|GetBuildPreview)
              (:then
                _)
              (:else))))
        (Actor|DestroyActor _buildpreview)))))

(fn BuildModeClient
  (params (StructureID :type Integer))
  (bind _buildpreview (Variables|Default|GetBuildPreview))
  (bind _buildpreview_2 (Variables|Default|GetBuildPreview))
  (bind _buildableinfo (Variables|/Game/_Main/Blueprints/BuildingSystem/BP_BuildableMaster.BP_BuildableMaster_C|GetBuildableInfo _buildpreview))
  (bind _buildableinfo_2 (Variables|/Game/_Main/Blueprints/BuildingSystem/BP_BuildableMaster.BP_BuildableMaster_C|GetBuildableInfo _buildpreview_2))
  (bind _survivalcharref (Class|BPISurvivalCharacter|GetSurvivalCharRef(Message) (Components|GetOwner)))
  (Variables|Default|GetBuildPreview
    (:then
      _)
    (:else
      (CallFunction|SpawnBuildPreview StructureID)
      (bind _buildpreview_3 (Variables|Default|GetBuildPreview)
        (:then
          _)
        (:else))))
  (bind (_outhit _returnvalue) (Collision|LineTraceByChannel (+ (Transformation|GetWorldLocation (Variables|/Game/_Main/Blueprints/Character/BP_FirstPersonMan.BP_FirstPersonMan_C|GetFirstPersonCamera _survivalcharref)) (* (Math|Vector|GetForwardVector (Variables|/Game/_Main/Blueprints/Character/BP_FirstPersonMan.BP_FirstPersonMan_C|GetFirstPersonCamera _survivalcharref)) (LocalVariables|GetBuildDistanceClose))) (+ (Transformation|GetWorldLocation (Variables|/Game/_Main/Blueprints/Character/BP_FirstPersonMan.BP_FirstPersonMan_C|GetFirstPersonCamera _survivalcharref)) (* (Math|Vector|GetForwardVector (Variables|/Game/_Main/Blueprints/Character/BP_FirstPersonMan.BP_FirstPersonMan_C|GetFirstPersonCamera _survivalcharref)) (LocalVariables|GetBuidlDistanceFar))) (.tracechannel (Variables|/Game/_Main/Blueprints/BuildingSystem/BP_BuildableMaster.BP_BuildableMaster_C|GetBuildableInfo _buildpreview_3)) false (Utilities|Array|MakeArray _buildpreview_3) "None"))
  (if _returnvalue
    (Variables|Default|SetHit%20Actor (.HitActor (Collision|BreakHitResult _outhit)))
    (Variables|Default|SetHit%20Component (.HitComponent (Collision|BreakHitResult _outhit)))
    (bind _survivalcharref_2 (Class|BPISurvivalCharacter|GetSurvivalCharRef(Message) (Components|GetOwner)))
    (Variables|Default|SetBuildTransform (Math|Transform|MakeTransform (.ImpactPoint (Collision|BreakHitResult _outhit)) (Math|Rotator|MakeRotator 0.0 0.0 (+ (.yaw (Transformation|GetWorldRotation (Variables|/Game/_Main/Blueprints/Character/BP_FirstPersonMan.BP_FirstPersonMan_C|GetFirstPersonCamera _survivalcharref_2))) 9e+01)) "1.000000,1.000000,1.000000"))
    (Utilities|IsValid (Variables|Default|GetBuildPreview)
      (:Is%20Valid
        (bind (_found_ _location) (CallFunction|GetSnappingPoints))
        (if _found_
          (Variables|Default|SetBuildTransform _location)
          (if (.dofloatcheck? _buildableinfo_2)
            (bind _didhit_ (CallFunction|IsBuildFloating?))
            (bind _overlapping_ (CallFunction|CheckforOverlap))
            (CallFunction|SetPreviewColor (and (not _overlapping_) _didhit_))
            (CallFunction|BuildLoop)
            (elif (.doceillingcheck? _buildableinfo_2)
              (bind _canplace_ (Class|BPIBuildInterface|CanPlaceCeiling?(Message) (Variables|Default|GetBuildPreview)))
              (bind _overlapping__2 (CallFunction|CheckforOverlap))
              (CallFunction|SetPreviewColor (and (not _overlapping__2) _canplace_))
              (CallFunction|BuildLoop)
              (else
                (bind _overlapping__3 (CallFunction|CheckforOverlap))
                (CallFunction|SetPreviewColor (not _overlapping__3))
                (CallFunction|BuildLoop))))
          (elif (.canplaceonground? _buildableinfo)
            (bind _didhit__2 (CallFunction|IsBuildFloating?))
            (bind _overlapping__4 (CallFunction|CheckforOverlap))
            (if (and (not _overlapping__4) _didhit__2)
              (CallFunction|SetPreviewColor true)
              (CallFunction|BuildLoop)
              (else
                (if (.canplaceonfoundation? _buildableinfo) :!label _label
                  (bind _onfoundation_ (CallFunction|BuildonFoundation?))
                  (bind _overlapping__5 (CallFunction|CheckforOverlap))
                  (CallFunction|SetPreviewColor (and (not _overlapping__5) _onfoundation_))
                  (CallFunction|BuildLoop)
                  (else
                    (CallFunction|SetPreviewColor false)
                    (CallFunction|BuildLoop)))))
            (else
              (goto _label)))))
      (:Is%20Not%20Valid
        (CallFunction|SpawnBuildPreview)
        (CallFunction|BuildLoop)))
    (else
      (bind _survivalcharref_3 (Class|BPISurvivalCharacter|GetSurvivalCharRef(Message) (Components|GetOwner)))
      (Variables|Default|SetBuildTransform (Math|Transform|MakeTransform (.TraceEnd (Collision|BreakHitResult _outhit)) (Math|Rotator|MakeRotator 0.0 0.0 (+ (.yaw (Transformation|GetWorldRotation (Variables|/Game/_Main/Blueprints/Character/BP_FirstPersonMan.BP_FirstPersonMan_C|GetFirstPersonCamera _survivalcharref_3))) 9e+01)) "1.000000,1.000000,1.000000"))
      (Utilities|IsValid (Variables|Default|GetBuildPreview)
        (:Is%20Valid
          (CallFunction|SetPreviewColor false)
          (CallFunction|BuildLoop))
        (:Is%20Not%20Valid
          (CallFunction|SpawnBuildPreview)
          (CallFunction|BuildLoop))))))

(fn SpawnBuildPreview
  (params (StructureID :type Integer))
  (bind _returnvalue (Utilities|GetDataTableRow "/Game/_Main/Blueprints/BuildingSystem/Misc/DT_Structures.DT_Structures" (Utilities|String|StringToName (Utilities|String|ToString(Integer) StructureID)))
    (:then
      (bind _returnvalue_2 (Game|SpawnActorfromClass (Utilities|Struct|BreakS_BuildTableInfo _returnvalue) (Variables|Default|GetBuildTransform) "Undefined" 0 0))
      (bind _output_get (Variables|Default|SetBuildPreview _returnvalue_2))
      (Collision|SetCollisionEnabled (Variables|/Game/_Main/Blueprints/BuildingSystem/BP_BuildableMaster.BP_BuildableMaster_C|GetStaticMesh _output_get) "NoCollision"))))

(fn SetPreviewColor
  (params (IsGreen? :type Boolean))
  (LocalVariables|SetLocalCanPlace? IsGreen?)
  (for _array_element (Actor|GetComponentsByClass (Variables|Default|GetBuildPreview) "/Script/Engine.StaticMeshComponent")
    (for _index (range 0 (- (Rendering|Material|GetNumMaterials _array_element) 1))
      (if (LocalVariables|GetLocalCanPlace?)
        (Rendering|Material|SetMaterial _array_element _index "/Game/_Main/Blueprints/BuildingSystem/Materials/M_Green.M_Green")
        (else
          (Rendering|Material|SetMaterial _array_element _index "/Game/_Main/Blueprints/BuildingSystem/Materials/M_Red.M_Red"))))
    (Transformation|SetWorldTransform (Variables|/Game/_Main/Blueprints/BuildingSystem/BP_BuildableMaster.BP_BuildableMaster_C|GetDefaultSceneRoot (Variables|Default|GetBuildPreview)) (Variables|Default|GetBuildTransform) false false)))

(fn SpawnBuildable
  (params (Transform :type Transform) (BuildIDTemp :type Integer))
  (LocalVariables|SetLocalTransfrom Transform)
  (bind _returnvalue (Utilities|GetDataTableRow "/Game/_Main/Blueprints/BuildingSystem/Misc/DT_Structures.DT_Structures" (Utilities|String|StringToName (Utilities|String|ToString(Integer) BuildIDTemp)))
    (:then
      (Game|SpawnActorfromClass (Utilities|Struct|BreakS_BuildTableInfo _returnvalue) (LocalVariables|GetLocalTransfrom) "Undefined" 0 0))))

(fn CheckforOverlap
  (bind _buildpreview (Variables|Default|GetBuildPreview))
  (bind _overlapboxsize (Variables|/Game/_Main/Blueprints/BuildingSystem/BP_BuildableMaster.BP_BuildableMaster_C|GetOverlapBoxSize _buildpreview))
  (bind _origin (Collision|GetComponentBounds _overlapboxsize))
  (bind _returnvalue (Collision|BoxTraceByChannel _origin _origin (Variables|/Script/Engine.BoxComponent|GetBoxExtent _overlapboxsize) (Math|Rotator|MakeRotator 0.0 0.0 (.yaw (Transformation|GetWorldRotation (Variables|/Script/Engine.Actor|GetRootComponent (Variables|Default|GetBuildPreview))))) "TraceTypeQuery1" false (Utilities|Array|MakeArray (Variables|Default|GetBuildPreview)) "None"))
  (return _returnvalue))

(fn BuildPlacementCheck
  (params (StructureID :type Integer) (ClientCameraVector :type Vector) (ClientCameraRotation :type Rotator))
  (bind _buildpreview (Variables|Default|GetBuildPreview))
  (bind _buildpreview_2 (Variables|Default|GetBuildPreview))
  (bind _buildableinfo (Variables|/Game/_Main/Blueprints/BuildingSystem/BP_BuildableMaster.BP_BuildableMaster_C|GetBuildableInfo _buildpreview_2))
  (bind _buildableinfo_2 (Variables|/Game/_Main/Blueprints/BuildingSystem/BP_BuildableMaster.BP_BuildableMaster_C|GetBuildableInfo _buildpreview))
  (bind _survivalcharref (Class|BPISurvivalCharacter|GetSurvivalCharRef(Message) (Components|GetOwner)))
  (LocalVariables|SetLocalCameraRotation ClientCameraRotation)
  (CallFunction|SpawnBuildPreview StructureID)
  (bind _buildpreview_3 (Variables|Default|GetBuildPreview)
    (:then
      (bind (_outhit _returnvalue) (Collision|LineTraceByChannel (+ (Transformation|GetWorldLocation (Variables|/Game/_Main/Blueprints/Character/BP_FirstPersonMan.BP_FirstPersonMan_C|GetFirstPersonCamera _survivalcharref)) (* ClientCameraVector (LocalVariables|GetBuildDistanceClose))) (+ (Transformation|GetWorldLocation (Variables|/Game/_Main/Blueprints/Character/BP_FirstPersonMan.BP_FirstPersonMan_C|GetFirstPersonCamera _survivalcharref)) (* ClientCameraVector (LocalVariables|GetBuildDistanceFar))) (.tracechannel (Variables|/Game/_Main/Blueprints/BuildingSystem/BP_BuildableMaster.BP_BuildableMaster_C|GetBuildableInfo _buildpreview_3)) false (Utilities|Array|MakeArray _buildpreview_3) "None"))
      (if _returnvalue
        (Variables|Default|SetHit%20Actor (.HitActor (Collision|BreakHitResult _outhit)))
        (Variables|Default|SetHit%20Component (.HitComponent (Collision|BreakHitResult _outhit)))
        (Variables|Default|SetBuildTransform (Math|Transform|MakeTransform (.ImpactNormal (Collision|BreakHitResult _outhit)) (Math|Rotator|MakeRotator 0.0 0.0 (+ (.Yaw (Math|Rotator|BreakRotator (LocalVariables|GetLocalCameraRotation))) 9e+01)) "1.000000,1.000000,1.000000"))
        (Utilities|IsValid (Variables|Default|GetBuildPreview)
          (:Is%20Valid
            (bind (_found_ _location) (CallFunction|GetSnappingPoints))
            (if _found_
              (Variables|Default|SetBuildTransform _location)
              (if (.dofloatcheck? _buildableinfo)
                (bind _didhit_ (CallFunction|IsBuildFloating?))
                (bind _overlapping_ (CallFunction|CheckforOverlap))
                (return (and (not _overlapping_) _didhit_))
                (elif (.doceillingcheck? _buildableinfo)
                  (bind _canplace_ (Class|BPIBuildInterface|CanPlaceCeiling?(Message) (Variables|Default|GetBuildPreview)))
                  (bind _overlapping__2 (CallFunction|CheckforOverlap))
                  (return (and (not _overlapping__2) _canplace_))
                  (else
                    (bind _overlapping__3 (CallFunction|CheckforOverlap))
                    (return (not _overlapping__3)))))
              (else
                (if (.canplaceonground? _buildableinfo_2)
                  (bind _didhit__2 (CallFunction|IsBuildFloating?))
                  (bind _overlapping__4 (CallFunction|CheckforOverlap))
                  (if (and (not _overlapping__4) _didhit__2)
                    (return true)
                    (else
                      _)))
                (if (.canplaceonfoundation? _buildableinfo_2)
                  (bind _overlapping__5 (CallFunction|CheckforOverlap))
                  (bind _onfoundation_ (CallFunction|BuildonFoundation?))
                  (return (and _onfoundation_ (not _overlapping__5)))
                  (else
                    (return false))))))
          (:Is%20Not%20Valid
            _))
        (else
          (Variables|Default|SetBuildTransform (Math|Transform|MakeTransform (.TraceEnd (Collision|BreakHitResult _outhit)) (Math|Rotator|MakeRotator 0.0 0.0 (+ (.Yaw (Math|Rotator|BreakRotator (LocalVariables|GetLocalCameraRotation))) 9e+01)) "1.000000,1.000000,1.000000"))
          (Utilities|IsValid (Variables|Default|GetBuildPreview)
            (:Is%20Valid
              _)
            (:Is%20Not%20Valid
              _))))
      (return false))
    (:else)))

(fn GetSnappingPoints
  (bind _boxes (Class|BPIBuildInterface|ReturnBoxes(Message) (Variables|Default|GetHit%20Actor)))
  (bind _array_element (Utilities|Array|ForEachLoopwithBreak _boxes :!label _label)
    (:LoopBody
      (bind _hit_component (Variables|Default|GetHit%20Component)
        (:then
          (if (== _array_element _hit_component)
            (LocalVariables|SetLocalFound? true)
            (goto _label Break)))
        (:else)))
    (:Completed
      (bind _hit_component_2 (Variables|Default|GetHit%20Component)
        (:then
          (return (LocalVariables|GetLocalFound?) (Transformation|GetWorldTransform _hit_component_2)))
        (:else
          (return (LocalVariables|GetLocalFound?) ""))))))

(fn ChangeBuildStructure
  (bind _buildpreview (Variables|Default|GetBuildPreview)
    (:then
      (Actor|DestroyActor _buildpreview))
    (:else
      _))
  (CallFunction|SpawnBuildPreview (Variables|Default|GetStructureIdDebug)))

(fn IsBuildFloating?
  (bind _buildtransform (Variables|Default|GetBuildTransform))
  (bind _returnvalue (Collision|LineTraceByChannel (.location _buildtransform) (- (.location _buildtransform) "0,0,50.000000") "TraceTypeQuery1" false (Utilities|Array|MakeArray (Variables|Default|GetBuildPreview)) "ForDuration"))
  (return _returnvalue))

(fn BuildonFoundation?
  (bind _buildpreview (Variables|Default|GetBuildPreview))
  (bind _staticmesh (Variables|/Game/_Main/Blueprints/BuildingSystem/BP_BuildableMaster.BP_BuildableMaster_C|GetStaticMesh _buildpreview))
  (bind _returnvalue (Transformation|GetWorldLocation _staticmesh))
  (bind (_outhit _returnvalue_2) (Collision|LineTraceByChannel _returnvalue (- _returnvalue "0,0,50.000000") "TraceTypeQuery1" false (Utilities|Array|MakeArray (Variables|Default|GetBuildPreview)) "None"))
  (if _returnvalue_2
    (return (Actor|ActorHasTag (.HitActor (Collision|BreakHitResult _outhit)) "Foundation"))
    (else
      (return false))))