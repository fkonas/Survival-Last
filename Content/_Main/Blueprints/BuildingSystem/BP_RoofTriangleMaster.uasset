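; Master Blueprint for triangle roof pieces in the building system, handling cascading destruction of snapped roofs.
; On its first destroy event it runs the parent logic, then sends the same event to every BP_SmallRoofMaster overlapping RoofBox, and removes itself after a short delay.
; ReturnBoxes exposes both roof boxes, though the destruction cascade checks only RoofBox.
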(event EventStructureDestroyEvent
  (if (not (Variables|Default|GetIsDestroyed?))
    (Variables|Default|SetIsDestroyed? true)
    (|CallParentFunction)
    (CallFunction|DestroySnappedRoof)
    (Utilities|FlowControl|Delay 3.0)
    (Actor|DestroyActor)))

(fn ConstructionScript
  (|CallParentFunction))

(fn ReturnBoxes
  (return (Utilities|Array|MakeArray (Variables|Default|GetRoofBox) (Variables|Default|GetRoofBox1))))

(fn DestroySnappedRoof
  (bind _output_get (LocalVariables|SetRoofArray (Collision|GetOverlappingActors (Variables|Default|GetRoofBox) "/Game/_Main/Blueprints/BuildingSystem/BP_SmallRoofMaster.BP_SmallRoofMaster_C" :!class /Script/Engine.PrimitiveComponent)))
  (if (> (Utilities|Array|Length _output_get) 0)
    (for _array_element (LocalVariables|GetRoofArray)
      (Class|BPIBuildInterface|StructureDestroyEvent(Message) _array_element))
    (return)
    (else
      (return))))