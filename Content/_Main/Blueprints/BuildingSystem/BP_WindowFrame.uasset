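; BP_WindowFrame is a window frame piece in the building system that takes any window in it down when it is destroyed.
; Its destroy event calls the parent logic, then sends the destroy message to every BP_WindowMaster actor overlapping WindowFrameBox.
; ReturnBoxes exposes its window frame, ceiling, triangle ceiling and wall boxes, apparently as attachment points for other pieces.
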(event EventStructureDestroyEvent
  (|CallParentFunction)
  (CallFunction|DestroyWindow))

(fn ConstructionScript
  (|CallParentFunction))

(fn ReturnBoxes
  (return (Utilities|Array|MakeArray (Variables|Default|GetWindowFrameBox) (Variables|Default|GetCeil) (Variables|Default|GetCeil1) (Variables|Default|GetTriangleCeiling) (Variables|Default|GetTriangleCeiling1) (Variables|Default|GetWallBox) (Variables|Default|GetWallBox1) (Variables|Default|GetWallBox2))))

(fn DestroyWindow
  (bind _output_get (LocalVariables|SetActors (Collision|GetOverlappingActors (Variables|Default|GetWindowFrameBox) "/Game/_Main/Blueprints/BuildingSystem/BP_WindowMaster.BP_WindowMaster_C" :!class /Script/Engine.PrimitiveComponent)))
  (if (> (Utilities|Array|Length _output_get) 0)
    (for _array_element (LocalVariables|GetActors)
      (Class|BPIBuildInterface|StructureDestroyEvent(Message) _array_element))
    (return)
    (else
      (return))))