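; BP_FoundationMaster is the base foundation piece in the building system, providing snap boxes for neighboring foundations, triangle foundations, walls, ramps and stairs.
; ReturnBoxes exposes those boxes as one array.
; On destruction, a one-shot guard runs the parent logic, then cascades the destroy event to buildables overlapping CheckWallsTrace that carry the AboveFoundation tag.
; The foundation removes itself after a short delay.
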(event EventStructureDestroyEvent
  (if (not (Variables|Default|GetIsDestroyed?))
    (Variables|Default|SetIsDestroyed? true)
    (|CallParentFunction)
    (CallFunction|DestroySnappedStructures)
    (Utilities|FlowControl|Delay 3.0)
    (Actor|DestroyActor)))

(fn ConstructionScript
  (|CallParentFunction))

(fn ReturnBoxes
  (return (Utilities|Array|MakeArray (Variables|Default|GetFoundation) (Variables|Default|GetFoundation1) (Variables|Default|GetFoundation2) (Variables|Default|GetFoundation3) (Variables|Default|GetWall) (Variables|Default|GetWall1) (Variables|Default|GetWall2) (Variables|Default|GetWall3) (Variables|Default|GetTriangleFoundation) (Variables|Default|GetTriangleFoundation1) (Variables|Default|GetTriangleFoundation2) (Variables|Default|GetTriangleFoundation3) (Variables|Default|GetRamp) (Variables|Default|GetRamp1) (Variables|Default|GetRamp2) (Variables|Default|GetRamp3) (Variables|Default|GetStairsBox))))

(fn DestroySnappedStructures
  (bind _output_get (LocalVariables|SetOverlapBuildables (Collision|GetOverlappingActors (Variables|Default|GetCheckWallsTrace) "/Game/_Main/Blueprints/BuildingSystem/BP_BuildableMaster.BP_BuildableMaster_C" :!class /Script/Engine.PrimitiveComponent)))
  (if (> (Utilities|Array|Length _output_get) 0)
    (for _array_element (LocalVariables|GetOverlapBuildables)
      (if (Actor|ActorHasTag _array_element "AboveFoundation")
        (Class|BPIBuildInterface|StructureDestroyEvent(Message) _array_element)))
    (return)
    (else
      (return))))