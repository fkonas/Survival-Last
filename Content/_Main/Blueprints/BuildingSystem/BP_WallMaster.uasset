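; BP_WallMaster is the wall base in the building system, providing snap boxes and cascading destruction to attached pieces.
; ReturnBoxes exposes its ceiling, triangle ceiling, torch and wall boxes.
; On destruction, a one-time guard runs the parent logic, then overlap queries message buildables tagged AboveWall or AboveFoundation, plus overlapping torches, to destroy themselves.
; The wall actor is removed after a short delay.
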(event EventStructureDestroyEvent
  (if (not (Variables|Default|GetIsDestroyed?))
    (Variables|Default|SetIsDestroyed? true)
    (|CallParentFunction)
    (CallFunction|DestroySnappedStructures)
    (Utilities|FlowControl|Delay 3.0)
    (Actor|DestroyActor)))

(fn ConstructionScript
  (|CallParentFunction))

(fn ReturnBoxes
  (return (Utilities|Array|MakeArray (Variables|Default|GetCeil) (Variables|Default|GetCeil1) (Variables|Default|GetTriangleCeiling) (Variables|Default|GetTriangleCeiling1) (Variables|Default|GetTorchBox1) (Variables|Default|GetTorchBox) (Variables|Default|GetWallBox) (Variables|Default|GetWallBox1) (Variables|Default|GetWallBox2))))

(fn DestroySnappedStructures
  (bind _output_get (LocalVariables|SetOverlappingCeilings (Collision|GetOverlappingActors (Variables|Default|GetDemoCeilling) "/Game/_Main/Blueprints/BuildingSystem/BP_BuildableMaster.BP_BuildableMaster_C" :!class /Script/Engine.PrimitiveComponent)))
  (if (> (Utilities|Array|Length _output_get) 0)
    (for _array_element (LocalVariables|GetOverlappingCeilings)
      (if (or (Actor|ActorHasTag _array_element "AboveWall") (Actor|ActorHasTag _array_element "AboveFoundation"))
        (Class|BPIBuildInterface|StructureDestroyEvent(Message) _array_element))))
  (bind _output_get_2 (LocalVariables|SetOverlappingCeilings (Collision|GetOverlappingActors (Variables|Default|GetOverlapBoxSize) "/Game/_Main/Blueprints/BuildingSystem/BP_Torch.BP_Torch_C" :!class /Script/Engine.PrimitiveComponent)))
  (if (> (Utilities|Array|Length _output_get_2) 0)
    (for _array_element_2 (LocalVariables|GetOverlappingCeilings)
      (Class|BPIBuildInterface|StructureDestroyEvent(Message) _array_element_2))
    (return)
    (else
      (return))))