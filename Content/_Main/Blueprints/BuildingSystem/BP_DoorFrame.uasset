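; Door frame piece for the building system, extending a parent structure with boxes for a door, ceilings, triangle ceilings, torches and walls.
; ReturnBoxes exposes these boxes as one array.
; On destruction it runs the parent logic, then finds doors overlapping the door box and torches overlapping the four torch boxes, passing the destroy message on to each.
; An IsDestroyed guard exists in the event graph but is never run.
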(event EventStructureDestroyEvent
  (|CallParentFunction)
  (CallFunction|DestroyDoorStructures))

(fn ConstructionScript
  (|CallParentFunction))

(fn ReturnBoxes
  (return (Utilities|Array|MakeArray (Variables|Default|GetDoorBox) (Variables|Default|GetCeil) (Variables|Default|GetCeil1) (Variables|Default|GetTriangleCeiling) (Variables|Default|GetTriangleCeiling1) (Variables|Default|GetTorchBox) (Variables|Default|GetTorchBox1) (Variables|Default|GetTorchBox2) (Variables|Default|GetTorchBox3) (Variables|Default|GetWallBox) (Variables|Default|GetWallBox1) (Variables|Default|GetWallBox2))))

(fn DestroyDoorStructures
  (bind _output_get (LocalVariables|SetOverlappingActors (Collision|GetOverlappingActors (Variables|Default|GetDoorBox) "/Game/_Main/Blueprints/BuildingSystem/BP_DoorMaster.BP_DoorMaster_C" :!class /Script/Engine.PrimitiveComponent)))
  (if (> (Utilities|Array|Length _output_get) 0)
    (for _array_element (LocalVariables|GetOverlappingActors)
      (Class|BPIBuildInterface|StructureDestroyEvent(Message) _array_element)))
  (bind _output_get_2 (LocalVariables|SetOverlappingActors (Collision|GetOverlappingActors (Variables|Default|GetTorchBox) "/Game/_Main/Blueprints/BuildingSystem/BP_Torch.BP_Torch_C" :!class /Script/Engine.PrimitiveComponent)))
  (if (> (Utilities|Array|Length _output_get_2) 0)
    (for _array_element_2 (LocalVariables|GetOverlappingActors)
      (Class|BPIBuildInterface|StructureDestroyEvent(Message) _array_element_2)))
  (bind _output_get_3 (LocalVariables|SetOverlappingActors (Collision|GetOverlappingActors (Variables|Default|GetTorchBox1) "/Game/_Main/Blueprints/BuildingSystem/BP_Torch.BP_Torch_C" :!class /Script/Engine.PrimitiveComponent)))
  (if (> (Utilities|Array|Length _output_get_3) 0)
    (for _array_element_3 (LocalVariables|GetOverlappingActors)
      (Class|BPIBuildInterface|StructureDestroyEvent(Message) _array_element_3)))
  (bind _output_get_4 (LocalVariables|SetOverlappingActors (Collision|GetOverlappingActors (Variables|Default|GetTorchBox2) "/Game/_Main/Blueprints/BuildingSystem/BP_Torch.BP_Torch_C" :!class /Script/Engine.PrimitiveComponent)))
  (if (> (Utilities|Array|Length _output_get_4) 0)
    (for _array_element_4 (LocalVariables|GetOverlappingActors)
      (Class|BPIBuildInterface|StructureDestroyEvent(Message) _array_element_4)))
  (bind _output_get_5 (LocalVariables|SetOverlappingActors (Collision|GetOverlappingActors (Variables|Default|GetTorchBox3) "/Game/_Main/Blueprints/BuildingSystem/BP_Torch.BP_Torch_C" :!class /Script/Engine.PrimitiveComponent)))
  (if (> (Utilities|Array|Length _output_get_5) 0)
    (for _array_element_5 (LocalVariables|GetOverlappingActors)
      (Class|BPIBuildInterface|StructureDestroyEvent(Message) _array_element_5))
    (return)
    (else
      (return))))