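; Triangular ceiling piece for the building system, exposing wall, ceiling and triangle-ceiling snap boxes through ReturnBoxes.
; Placement is allowed only when its lower box overlaps at least one wall.
; On destruction it guards against repeats, runs the parent logic, then propagates destruction to overlapping buildables tagged AboveFoundation, cascading collapse before removing itself after a short delay.
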(event EventStructureDestroyEvent
  (if (not (Variables|Default|GetIsDestroyed?))
    (Variables|Default|SetIsDestroyed? true)
    (|CallParentFunction)
    (CallFunction|DestroySnappedStructures)
    (Utilities|FlowControl|Delay 3.0)
    (Actor|DestroyActor)))

(fn ConstructionScript
  (|CallParentFunction))

(fn ReturnBoxes
  (return (Utilities|Array|MakeArray (Variables|Default|GetWall) (Variables|Default|GetWall1) (Variables|Default|GetWall2) (Variables|Default|GetCeiling) (Variables|Default|GetCeiling1) (Variables|Default|GetCeiling2) (Variables|Default|GetTriangleCeiling) (Variables|Default|GetTriangleCeiling1) (Variables|Default|GetTriangleCeiling2))))

(fn DestroySnappedStructures
  (bind _output_get (LocalVariables|SetActors (Collision|GetOverlappingActors (Variables|Default|GetDestroyBox) "/Game/_Main/Blueprints/BuildingSystem/BP_BuildableMaster.BP_BuildableMaster_C" :!class /Script/Engine.PrimitiveComponent)))
  (if (> (Utilities|Array|Length _output_get) 0)
    (for _array_element (LocalVariables|GetActors)
      (if (Actor|ActorHasTag _array_element "AboveFoundation")
        (Class|BPIBuildInterface|StructureDestroyEvent(Message) _array_element)))
    (return)
    (else
      (return))))

(fn CanPlaceCeiling?
  (return (> (Utilities|Array|Length (Collision|GetOverlappingActors (Variables|Default|GetBellowBox) "/Game/_Main/Blueprints/BuildingSystem/BP_WallMaster.BP_WallMaster_C" :!class /Script/Engine.PrimitiveComponent)) 0)))