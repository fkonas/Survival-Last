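; Placeable smelting forge for the building system that turns items in its storage container into recipe outputs while lit.
; LightFireStructure toggles the fire effect and a looping timer, lighting only if the container holds fuel (item ID 1).
; Each tick crafts every satisfiable DT_ForgeRecipes row once, pulling outputs from DT_Items.
; It then burns one fuel, or extinguishes the fire when none remains.
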(event Custom|ShowFireFX
  (params (NewVisibility :type Boolean))
  ;[0 0 0] Show Fire FX
  (Rendering|SetVisibility (Variables|Default|GetFire) NewVisibility false))

(event Custom|CookItemsLoop
  ;[0 0 0] Smelt Item Loop
  (bind _returnvalue (Utilities|Time|SetTimerbyEvent (delegate Custom|SmeltItems) 15.0 true))
  (Variables|Default|SetTimerRef _returnvalue))

(event Custom|SmeltItems
  ;[0 0 0] Check if we can craft items.
  (bind _outrownames (DataTable|GetDataTableRowNames "/Game/_Main/Blueprints/DataTables/DT_ForgeRecipes.DT_ForgeRecipes"))
  (for _array_element _outrownames
    (bind _returnvalue (Utilities|GetDataTableRow "/Game/_Main/Blueprints/DataTables/DT_ForgeRecipes.DT_ForgeRecipes" _array_element)
      (:then
        (Variables|Default|SetItemName (Utilities|String|StringToName (Utilities|String|ToString(Integer) (.ItemID (Utilities|Struct|BreakS_ItemRecipe _returnvalue)))))
        (Variables|Default|SetRequired%20Items (.RequiredItems (Utilities|Struct|BreakS_ItemRecipe _returnvalue)))
        (bind _cancraft_ (Default|ContainsItems (Variables|Default|GetBPC_StorageContainer) (.RequiredItems (Utilities|Struct|BreakS_ItemRecipe _returnvalue))))
        (if _cancraft_
          (Default|RemoveItems (Variables|Default|GetBPC_StorageContainer) (Variables|Default|GetRequired%20Items))
          (bind _returnvalue_2 (Utilities|GetDataTableRow "/Game/_Main/Blueprints/DataTables/DT_Items.DT_Items" (Variables|Default|GetItemName))
            (:then
              (Default|AddItemonServer (Variables|Default|GetBPC_StorageContainer) _returnvalue_2)))))))
  (bind _cancraft__2 (Default|ContainsItems (Variables|Default|GetBPC_StorageContainer) (Utilities|Array|MakeArray (Utilities|Struct|MakeS_ItemStruct 1 1))))
  (if _cancraft__2
    (Default|RemoveItems (Variables|Default|GetBPC_StorageContainer) (Utilities|Array|MakeArray (Utilities|Struct|MakeS_ItemStruct 1 1)))
    (else
      (bind _output_get (Variables|Default|SetFireOn? false))
      (CallFunction|ShowFireFX _output_get)
      (Utilities|Time|ClearandInvalidateTimerbyHandle (Variables|Default|GetTimerRef)))))

(event EventLightFireStructure
  ;[0 0 0] Light Fire Button
  (if (Variables|Default|GetFireOn?)
    (bind _output_get (Variables|Default|SetFireOn? false))
    (CallFunction|ShowFireFX _output_get)
    (Utilities|Time|ClearandInvalidateTimerbyHandle (Variables|Default|GetTimerRef))
    (else
      (bind _cancraft_ (Default|ContainsItems (Variables|Default|GetBPC_StorageContainer) (Utilities|Array|MakeArray (Utilities|Struct|MakeS_ItemStruct 1 1))))
      (if _cancraft_
        (bind _output_get_2 (Variables|Default|SetFireOn? true))
        (CallFunction|ShowFireFX _output_get_2)
        (CallFunction|CookItemsLoop)))))

(fn ConstructionScript
  (|CallParentFunction))