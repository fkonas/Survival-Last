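; BP_InventoryBag is an inventory bag under placeable structures that removes itself from the world after a time.
; On BeginPlay the server starts a one-shot five-minute timer, and DestroyBagEvent can trigger the same teardown on demand.
; Teardown blocks further access, calls RemoveAllCharacters, then destroys the actor after a short delay.
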(event Custom|DestroySelf
  (Variables|Default|SetCantAccess? true)
  (CallFunction|RemoveAllCharacters)
  (Utilities|FlowControl|Delay 0.5)
  (Actor|DestroyActor))

(event EventBeginPlay
  (Networking|SwitchHasAuthority
    (:Authority
      (Utilities|Time|SetTimerbyEvent (delegate Custom|DestroySelf) 3e+02))))

(event EventDestroyBagEvent
  (CallFunction|DestroySelf))

(fn ConstructionScript
  (|CallParentFunction))