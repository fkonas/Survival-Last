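; BP_StorageCrate is a placeable storage crate in the building system that animates when its storage is opened or closed.
; The open and close storage events each call a multicast event, so the animation is intended to play for all clients.
; Opening plays one timeline from the start and closing plays a second in reverse from the end, both driving the roll of StaticMesh1, likely the lid.
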(event Custom|OpenBoxMulticast
  (bind _newtrack_0 (Timeline|Timeline_0 PlayFromStart)
    (:Update
      (Transformation|SetRelativeRotation (Variables|Default|GetStaticMesh1) (Math|Rotator|MakeRotator _newtrack_0 0.0 0.0) false false))))

(event Custom|CloseBoxMulticast
  (bind _newtrack_0 (Timeline|Timeline_1 ReverseFromEnd)
    (:Update
      (Transformation|SetRelativeRotation (Variables|Default|GetStaticMesh1) (Math|Rotator|MakeRotator _newtrack_0 0.0 0.0) false false))))

(event EventCloseStorageEvent
  (CallFunction|CloseBoxMulticast))

(event EventOpenStorageEvent
  (CallFunction|OpenBoxMulticast))

(fn ConstructionScript
  (|CallParentFunction))