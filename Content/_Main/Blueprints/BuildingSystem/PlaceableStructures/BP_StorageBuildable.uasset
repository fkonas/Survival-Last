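; Base placeable storage structure that players interact with to view a shared item container.
; It tracks accessing characters, opening on the first and closing on the last, and pushes slot changes from BPCStorageContainer to each viewer's player controller UI.
; On destruction it locks access, hides viewers' widgets and, depending on IsBagEmpty, moves items into a spawned BP_InventoryBag.
; UI refreshes also run an IsBagEmpty check that can fire DestroyBagEvent.
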(event Custom|AccessStorageBox
  (params (Character :type BP%20First%20Person%20Man%20Object%20Reference))
  ;[1 1 1] Play Open Storage Box Animation
  (bind _isaccessed_ (CallFunction|StorageBoxEvent))
  (if _isaccessed_
    _
    (else
      (CallFunction|OpenStorageEvent)))
  (bind _controllerref (Class|BPISurvivalCharacter|GetControllerfromCharacter(Message) Character))
  (bind _playercontrollerref (Class|BPISurvivalLostPC|SurvivalLostPCRef(Message) _controllerref))
  (Default|ShowStorageWidget _playercontrollerref (Utilities|Array|Length (Variables|/Game/_Main/Blueprints/Inventory/BPC_ItemContainer.BPC_ItemContainer_C|GetItems (Variables|Default|GetBPC_StorageContainer))) (Variables|Default|GetStorage%20Type))
  ;[0 0 0] Display Widgets, Update Slots and Text
  (Utilities|Array|Add (Variables|Default|GetAccessingCharacter) Character)
  (for (_array_element _array_index) (Variables|/Game/_Main/Blueprints/Inventory/BPC_ItemContainer.BPC_ItemContainer_C|GetItems (Variables|Default|GetBPC_StorageContainer))
    (if (== (Utilities|Struct|BreakS_ItemInfo _array_element) 0)
      (Default|ResetItemSlot _playercontrollerref "NewEnumerator2" _array_index)
      (else
        (Default|UpdateItemSlot _playercontrollerref "NewEnumerator2" _array_index _array_element)))))

(event Custom|UpdateWidgets
  (params (Container :type E_ContainerType%20Enum :default "NewEnumerator0") (Index :type Integer) (ItemInfo :type S%20Item%20Info%20Structure))
  ;[0 0 0] Update Widgets For Players Viewing Storage Container
  (for _array_element (Variables|Default|GetAccessingCharacter)
    (Utilities|IsValid _array_element
      (:Is%20Valid
        (bind _playercontrollerref (Class|BPISurvivalLostPC|SurvivalLostPCRef(Message) (Pawn|GetController _array_element)))
        (if (== (Utilities|Struct|BreakS_ItemInfo ItemInfo) 0)
          (Default|ResetItemSlot _playercontrollerref Container Index)
          (else
            (Default|UpdateItemSlot _playercontrollerref Container Index ItemInfo)))))))

(event Custom|ResetItemSlot
  (params (Container :type E_ContainerType%20Enum :default "NewEnumerator0") (Index :type Integer))
  ;[0 0 0] Update Widgets For Players Viewing Storage Container
  (for _array_element (Variables|Default|GetAccessingCharacter)
    (Utilities|IsValid _array_element
      (:Is%20Valid
        (bind _playercontrollerref (Class|BPISurvivalLostPC|SurvivalLostPCRef(Message) (Pawn|GetController _array_element)))
        (Default|ResetItemSlot _playercontrollerref Container Index)))))

(event Custom|UpdateStorageUI
  ;[0 0 0] Reset Storage Box Window
  (for _array_element (Variables|Default|GetAccessingCharacter)
    (Utilities|IsValid _array_element
      (:Is%20Valid
        (bind _playercontrollerref (Class|BPISurvivalLostPC|SurvivalLostPCRef(Message) (Pawn|GetController _array_element)))
        (Default|UpdateStorageSlots _playercontrollerref (Utilities|Array|Length (Variables|/Game/_Main/Blueprints/Inventory/BPC_ItemContainer.BPC_ItemContainer_C|GetItems (Variables|Default|GetBPC_StorageContainer))))
        (for (_array_element_2 _array_index) (Variables|/Game/_Main/Blueprints/Inventory/BPC_ItemContainer.BPC_ItemContainer_C|GetItems (Variables|Default|GetBPC_StorageContainer))
          (if (== (Utilities|Struct|BreakS_ItemInfo _array_element_2) 0)
            (Default|ResetItemSlot _playercontrollerref "NewEnumerator2" _array_index)
            (else
              (Default|UpdateItemSlot _playercontrollerref "NewEnumerator2" _array_index _array_element_2)))))))
  (CallFunction|DestroyBagifEmpty))

(event Custom|RemoveFromBox
  (params (Character :type BP%20First%20Person%20Man%20Object%20Reference))
  (Utilities|Array|RemoveItem (Variables|Default|GetAccessingCharacter) Character)
  (bind _isaccessed_ (CallFunction|StorageBoxEvent))
  (if (not _isaccessed_)
    (CallFunction|CloseStorageEvent)))

(event Custom|RemoveAllCharacters
  ;[0 0 0] Hide Storage widget for all players who are accessing it
  (for _array_element (Variables|Default|GetAccessingCharacter)
    (Utilities|IsValid _array_element
      (:Is%20Valid
        (bind _controllerref (Class|BPISurvivalCharacter|GetControllerfromCharacter(Message) _array_element))
        (bind _playercontrollerref (Class|BPISurvivalLostPC|SurvivalLostPCRef(Message) _controllerref))
        (Default|ShowStorageWidget _playercontrollerref 0 "NewEnumerator0")))))

(event Custom|DestroyBagIfEmpty
  ;[0 0 0] Hide Storage Widget For All Players Who Are Accessing It
  (bind _containsitem_ (Default|IsBagEmpty? (Variables|Default|GetBPC_StorageContainer)))
  (if (not _containsitem_)
    (CallFunction|DestroyBagEvent)))

(event EventStructureDestroyEvent
  ;[0 0 0] Show Destructable Mesh, Remove all Accessing Characters, and Spawn in Inventory Bag
  (|CallParentFunction)
  (Variables|Default|SetCantAccess? true)
  (CallFunction|RemoveAllCharacters)
  (Utilities|FlowControl|Delay 2.5)
  (bind _containsitem_ (Default|IsBagEmpty? (Variables|Default|GetBPC_StorageContainer)))
  (if _containsitem_
    (bind _returnvalue (Game|SpawnActorfromClass "/Game/_Main/Blueprints/BuildingSystem/PlaceableStructures/BP_InventoryBag.BP_InventoryBag_C" (Math|Transform|MakeTransform (Transformation|GetActorLocation) "0, 0, 0" "1.000000,1.000000,1.000000") "Undefined" 0 0))
    (bind _items (Default|GetAllItems (Variables|Default|GetBPC_StorageContainer)))
    (Utilities|Array|AppendArray (Variables|/Game/_Main/Blueprints/Inventory/BPC_ItemContainer.BPC_ItemContainer_C|GetItems (Variables|BP_StorageBuildable_C|GetBPC_StorageContainer _returnvalue)) _items)
    (Utilities|FlowControl|Delay 0.5)
    (Actor|DestroyActor)
    (else
      (Actor|DestroyActor))))

(event EventInteractEvent
  (params (CharRef :type BP%20First%20Person%20Man%20Object%20Reference))
  (if (not (Variables|Default|GetCantAccess?))
    (bind _survivalcharref (Class|BPISurvivalCharacter|GetSurvivalCharRef(Message) CharRef))
    (Default|StorageBoxAccess _survivalcharref self)))

(fn ConstructionScript
  (|CallParentFunction))

(fn StorageBoxEvent
  (bind _output_get (Variables|Default|SetIsAccessed? (> (Utilities|Array|Length (Variables|Default|GetAccessingCharacter)) 0)))
  (return _output_get))

(fn GetStorageReference
  (return self))