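; BP_RoofLeftMaster is the master Blueprint for left roof pieces in the building system, extending a parent structure class.
; On its first destroy event it runs the parent logic, cascades destruction to large roof pieces overlapping RoofBox, then removes itself after a short delay.
; The cascade messages each BP_RoofLargeMaster as destroyed rather than demolished, with no player name.
; ReturnBoxes exposes RoofBox as the piece's only box.
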(event EventStructureDestroyEvent
  (params (DemolishedOrDestroyed? :type Boolean) (PlayerName :type Text))
  (if (not (Variables|Default|GetIsDestroyed?))
    (Variables|Default|SetIsDestroyed? true)
    (|CallParentFunction DemolishedOrDestroyed? PlayerName)
    (CallFunction|DestroySnappedRoof)
    (Utilities|FlowControl|Delay 3.0)
    (Actor|DestroyActor)))

(fn ConstructionScript
  (|CallParentFunction))

(fn ReturnBoxes
  (return (Utilities|Array|MakeArray (Variables|Default|GetRoofBox))))

(fn DestroySnappedRoof
  (bind _output_get (LocalVariables|SetLocalRoof (Collision|GetOverlappingActors (Variables|Default|GetRoofBox) "/Game/_Main/Blueprints/BuildingSystem/BP_RoofLargeMaster.BP_RoofLargeMaster_C" :!class /Script/Engine.PrimitiveComponent)))
  (if (> (Utilities|Array|Length _output_get) 0)
    (for _array_element (LocalVariables|GetLocalRoof)
      (Class|BPIBuildInterface|StructureDestroyEvent(Message) _array_element false))
    (return)
    (else
      (return))))