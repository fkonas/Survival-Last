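; BP_RoofLargeMaster is the base Blueprint for large roof pieces in the building system.
; On its destroy event it runs the parent handler once, guarded by an IsDestroyed flag, then removes the actor after a short delay.
; It overrides ReturnBoxes to supply its two roof box components to the building system.
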(event EventStructureDestroyEvent
  (if (not (Variables|Default|GetIsDestroyed?))
    (Variables|Default|SetIsDestroyed? true)
    (|CallParentFunction)
    (Utilities|FlowControl|Delay 3.0)
    (Actor|DestroyActor)))

(fn ConstructionScript
  (|CallParentFunction))

(fn ReturnBoxes
  (return (Utilities|Array|MakeArray (Variables|Default|GetRoofBox) (Variables|Default|GetRoofBox1))))