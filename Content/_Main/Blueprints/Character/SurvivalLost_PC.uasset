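; Player controller for a multiplayer survival game, acting as the hub between gameplay and the player's UI.
; BeginPlay creates the main widget only without authority; events relay inventory, storage, stats, armor, crafting and notifications into its child widgets.
; Tab or I toggles inventory, closing open storage and switching input mode.
; Tribe actions update PlayerState and call GameState through interface messages, with rank checks on management and leaving, then refresh the tribe window.
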(event Custom|InventoryOnClient
  ;[0 0 0] Show / Hide Inventory
  (if (Variables|Default|GetInventoryShown?)
    (Default|SetInventoryVis (Variables|Default|GetMainWidgetRef) false)
    (Variables|Default|SetbShowMouseCursor false)
    (Input|SetInputModeGameOnly self false)
    (Variables|Default|SetInventoryShown? false)
    (Default|CloseDropWindow (Variables|Default|GetMainWidgetRef))
    (else
      (Default|SetInventoryVis (Variables|Default|GetMainWidgetRef) true)
      (Variables|Default|SetbShowMouseCursor true)
      (Input|SetInputModeGameandUI self 0 "DoNotLock" true false)
      (Variables|Default|SetInventoryShown? true))))

(event Custom|ResetItemSlot
  (params (Container :type E_ContainerType%20Enum :default "NewEnumerator0") (Index :type Integer))
  (bind _widget (CallFunction|GetInventoryWidget Container Index))
  (Utilities|IsValid _widget
    (:Is%20Valid
      (Default|ResetSlot _widget))))

(event Custom|ExperienceNotify
  (params (Experience :type Integer))
  ;[1 1 1] Experience and Level Notifications
  (Default|AddExperienceNotification (Variables|Default|GetMainWidgetRef) Experience))

(event Custom|UpdateLevelUI
  (params (PlayerLevel :type Integer))
  ;[1 1 1] Experience and Level Notifications
  (Default|UpdatePlayerLevel (Variables|/Game/_Main/Widgets/W_MainWidget.W_MainWidget_C|GetW_Inventory (Variables|Default|GetMainWidgetRef)) PlayerLevel))

(event Custom|LevelNotify
  (params (Level :type Integer))
  ;[1 1 1] Experience and Level Notifications
  (Default|ShowLevelUpNotification (Variables|Default|GetMainWidgetRef) Level))

(event Custom|UpdateSkillPoints
  (params (SkillPoints :type Integer))
  ;[1 1 1] Experience and Level Notifications
  (Default|UpdateSkillPoints (Variables|/Game/_Main/Widgets/InventoryWidgets/W_Inventory.W_Inventory_C|GetW_PlayerInfoWindow (Variables|/Game/_Main/Widgets/W_MainWidget.W_MainWidget_C|GetW_Inventory (Variables|Default|GetMainWidgetRef))) SkillPoints))

(event Custom|RemoveLevelNotify
  ;[1 1 1] Experience and Level Notifications
  (Default|RemoveLevelUpNotification (Variables|Default|GetMainWidgetRef)))

(event Custom|UpdateArmorUI
  (params (ArmorType :type E_ArmorType%20Enum :default "NewEnumerator0") (ItemInfo :type S%20Item%20Info%20Structure))
  ;[1 1 1] Update Armor Widgets
  (Default|UpdateArmorSlot (Variables|/Game/_Main/Widgets/W_MainWidget.W_MainWidget_C|GetW_Inventory (Variables|Default|GetMainWidgetRef)) ArmorType ItemInfo))

(event Custom|RemoveArmorUI
  (params (ArmorType :type E_ArmorType%20Enum :default "NewEnumerator0"))
  ;[1 1 1] Update Armor Widgets
  (Default|RemoveArmorSlot (Variables|/Game/_Main/Widgets/W_MainWidget.W_MainWidget_C|GetW_Inventory (Variables|Default|GetMainWidgetRef)) ArmorType))

(event Custom|SetRenderMaterial
  (params (Mat :type Material%20Instance%20Object%20Reference))
  ;[1 1 1] Setup Player 2D Window Capture
  (Default|SetPlayerTexture (Variables|/Game/_Main/Widgets/W_MainWidget.W_MainWidget_C|GetW_Inventory (Variables|Default|GetMainWidgetRef)) Mat))

(event Custom|ShowStorageWidget
  (params (TotalSlots :type Integer) (StorageType :type E_CraftingType%20Enum :default "NewEnumerator0"))
  ;[0 0 0] Show / Hide Inventory
  (CallFunction|InventoryonClient)
  (if (Variables|Default|GetIsStorageShown?)
    (Default|SetStorageWindow (Variables|/Game/_Main/Widgets/W_MainWidget.W_MainWidget_C|GetW_Inventory (Variables|Default|GetMainWidgetRef)) 0 StorageType "Hidden")
    (Variables|Default|SetIsStorageShown? false)
    (bind _survivalcharref (Class|BPISurvivalCharacter|GetSurvivalCharRef(Message) (Pawn|GetControlledPawn)))
    (Default|RemoveReffromBox _survivalcharref)
    (else
      (Default|SetStorageWindow (Variables|/Game/_Main/Widgets/W_MainWidget.W_MainWidget_C|GetW_Inventory (Variables|Default|GetMainWidgetRef)) TotalSlots StorageType "Visible")
      (Variables|Default|SetIsStorageShown? true)
      (Class|WidgetSwitcher|SetActiveWidgetIndex (Variables|/Game/_Main/Widgets/InventoryWidgets/W_Inventory.W_Inventory_C|GetCraftingTableSwitcher (Variables|/Game/_Main/Widgets/W_MainWidget.W_MainWidget_C|GetW_Inventory (Variables|Default|GetMainWidgetRef)))))))

(event Custom|ShowOrHideInventory
  ;[0 0 0] Show / Hide Inventory
  (if (Variables|Default|GetInventoryShown?)
    (if (Variables|Default|GetIsStorageShown?)
      (CallFunction|ShowStorageWidget 0 "NewEnumerator0")
      (else
        (CallFunction|InventoryonClient :!label _label)))
    (else
      (goto _label))))

(event Custom|UpdateItemSlot
  (params (Container :type E_ContainerType%20Enum :default "NewEnumerator0") (Index :type Integer) (ItemInfo :type S%20Item%20Info%20Structure))
  (bind _widget (CallFunction|GetInventoryWidget Container Index))
  (Utilities|IsValid _widget
    (:Is%20Valid
      (Default|UpdateSlot _widget ItemInfo))))

(event Custom|UpdateStorageSlots
  (params (TotalSlots :type Integer))
  (Default|UpdateSlots (Variables|/Game/_Main/Widgets/InventoryWidgets/W_Inventory.W_Inventory_C|GetStorageBoxGrid (Variables|/Game/_Main/Widgets/W_MainWidget.W_MainWidget_C|GetW_Inventory (Variables|Default|GetMainWidgetRef))) TotalSlots))

(event Custom|ToggleMainWidget
  (params (WidgetToShow :type E_ToggleWidget%20Enum :default "NewEnumerator0"))
  (bind _playerstateref (Class|BPISurvivalPlayerState|GetPlayerStateRef(Message) (Variables|GetPlayerState)))
  (CallFunction|ToggleWidgetonClient WidgetToShow (Variables|/Game/_Main/Blueprints/GameModes/SurvivalGame_PlayerState.SurvivalGame_PlayerState_C|GetIsInTribe? _playerstateref)))

(event Custom|ToggleWidgetOnClient
  (params (WidgetToShow :type E_ToggleWidget%20Enum :default "NewEnumerator0") (IsInTribe? :type Boolean))
  (Default|ToggleWidgettoDisplay (Variables|Default|GetMainWidgetRef) WidgetToShow IsInTribe?))

(event Custom|CreateTribeOnServer
  (params (TribeName :type Text))
  ;[0 0 0] Tribe Basics: Create Tribe or Join Tribe
  (CallFunction|CreateTribeFunction TribeName))

(event Custom|UpdateTribeWindow
  (params (TribeInfo :type S%20Tribe%20Info%20Structure))
  ;[0 0 0] Update Tribe Window
  (Default|UpdateTribeWidget (Variables|/Game/_Main/Widgets/TribeWidgets/W_TribeSwitcher.W_TribeSwitcher_C|GetW_TribeWindow (Variables|/Game/_Main/Widgets/W_MainWidget.W_MainWidget_C|GetW_TribeSwitcher (Variables|Default|GetMainWidgetRef))) TribeInfo))

(event Custom|ShowTribeWindow
  ;[0 0 0] Update Tribe Window
  (Default|ShowTribeWindow (Variables|Default|GetMainWidgetRef)))

(event Custom|ShowTribeInviteWindow
  (params (TribeName :type Text) (SenderName :type Text))
  ;[0 0 0] Update Tribe Window
  (Default|ShowTribeInvite (Variables|Default|GetMainWidgetRef) SenderName TribeName))

(event Custom|RemoveTribeInviteBox
  ;[0 0 0] Update Tribe Window
  (Default|RemoveTribeInvite (Variables|Default|GetMainWidgetRef)))

(event Custom|JoinTribe
  (params (TribeID :type String) (WhoInvited :type Text))
  ;[0 0 0] Tribe Basics: Create Tribe or Join Tribe
  (CallFunction|JoinTribeFunction TribeID WhoInvited))

(event Custom|UpdateTribeMemmbers
  (params (TribeMemberArray :type Array%20of%20S%20Tribe%20Member%20Info%20Structures))
  (bind _mainwidgetref (Variables|Default|GetMainWidgetRef))
  (bind _w_tribeswitcher (Variables|/Game/_Main/Widgets/W_MainWidget.W_MainWidget_C|GetW_TribeSwitcher _mainwidgetref))
  (bind _w_tribewindow (Variables|/Game/_Main/Widgets/TribeWidgets/W_TribeSwitcher.W_TribeSwitcher_C|GetW_TribeWindow _w_tribeswitcher))
  ;[0 0 0] Update Tribe Window
  (Variables|/Game/_Main/Widgets/TribeWidgets/W_TribeWindow.W_TribeWindow_C|SetTribe%20Members _w_tribewindow TribeMemberArray)
  (Default|UpdateTribeMBox _w_tribewindow))

(event Custom|ShowItemWidget
  (params (ResourceImage :type Texture%202D%20Object%20Reference) (ResourceQunatity :type Integer) (ResourceName :type Text))
  (Default|ShowItemCollected (Variables|Default|GetMainWidgetRef) ResourceImage ResourceQunatity ResourceName))

(event Custom|UpdateTribeLogUI
  (params (TribeLogEvent :type S%20Tribe%20Log%20Entry%20Structure))
  ;[0 0 0] Update Tribe Window
  (Default|AddLogEvent (Variables|/Game/_Main/Widgets/TribeWidgets/W_TribeSwitcher.W_TribeSwitcher_C|GetW_TribeWindow (Variables|/Game/_Main/Widgets/W_MainWidget.W_MainWidget_C|GetW_TribeSwitcher (Variables|Default|GetMainWidgetRef))) TribeLogEvent))

(event Custom|UpdateTribeButtons
  (params (TribeRank :type E_TribeRank%20Enum :default "NewEnumerator0"))
  ;[0 0 0] Update Tribe Window
  (Default|SetTribeButtons (Variables|/Game/_Main/Widgets/TribeWidgets/W_TribeSwitcher.W_TribeSwitcher_C|GetW_TribeWindow (Variables|/Game/_Main/Widgets/W_MainWidget.W_MainWidget_C|GetW_TribeSwitcher (Variables|Default|GetMainWidgetRef))) TribeRank))

(event Custom|DemoteTribeMember
  (params (TribeMemberID :type String))
  (CallFunction|DemoteMemberFunction TribeMemberID))

(event Custom|KickTribeMember
  (params (TribeMemberID :type String))
  (CallFunction|KickMemberFunction TribeMemberID))

(event Custom|LeaveTribe
  (CallFunction|LeaveTribeFunction))

(event Custom|PromoteTribeMember
  (params (TribeMemberID :type String))
  (CallFunction|PromoteMemberFunction TribeMemberID))

(event Custom|UpdateTribeRank
  (params (Rank :type E_TribeRank%20Enum :default "NewEnumerator0"))
  (bind _playerstateref (Class|BPISurvivalPlayerState|GetPlayerStateRef(Message) (Variables|GetPlayerState)))
  (bind _output_get (Variables|/Game/_Main/Blueprints/GameModes/SurvivalGame_PlayerState.SurvivalGame_PlayerState_C|SetTribeRank _playerstateref Rank))
  (CallFunction|UpdateTribeButtons _output_get))

(event Custom|RemoveFromTribe
  (bind _playerstateref (Class|BPISurvivalPlayerState|GetPlayerStateRef(Message) (Variables|GetPlayerState)))
  (Variables|/Game/_Main/Blueprints/GameModes/SurvivalGame_PlayerState.SurvivalGame_PlayerState_C|SetIsInTribe? _playerstateref false)
  (Variables|/Game/_Main/Blueprints/GameModes/SurvivalGame_PlayerState.SurvivalGame_PlayerState_C|SetTribeID _playerstateref "")
  (Variables|/Game/_Main/Blueprints/GameModes/SurvivalGame_PlayerState.SurvivalGame_PlayerState_C|SetTribeName _playerstateref "")
  (CallFunction|ResetTribeWindow))

(event Custom|ResetTribeWindow
  (Default|ShowCreateATribeWindow (Variables|Default|GetMainWidgetRef)))

(event Custom|SetTribeMessage
  (params (MOTD :type Text))
  (bind (_tribeid _isintribe_ _playername _rank) (Class|BPISurvivalPlayerState|GetTribeID(Message) (Variables|GetPlayerState)))
  (if _isintribe_
    (if (or (Utilities|Enum|Equal(Enum) _rank "NewEnumerator0") (Utilities|Enum|Equal(Enum) _rank "NewEnumerator1"))
      (bind _gamestateref (Class|BPISurvivalGameState|GetGameStateRef(Message) (Game|GetGameState)))
      (Default|SetMOTD _gamestateref _tribeid MOTD _playername))))

(event Custom|UpdateCraftStatus
  (params (CanCratf? :type Boolean) (PlayerOrStorage? :type Boolean))
  (bind _mainwidgetref (Variables|Default|GetMainWidgetRef))
  (bind _w_inventory (Variables|/Game/_Main/Widgets/W_MainWidget.W_MainWidget_C|GetW_Inventory _mainwidgetref))
  (if PlayerOrStorage?
    (Default|UpdateCraftingStatus (Variables|/Game/_Main/Widgets/InventoryWidgets/W_Inventory.W_Inventory_C|GetW_CraftingWindow _w_inventory) CanCratf?)
    (else
      (Default|UpdateCraftingStatus (Variables|/Game/_Main/Widgets/InventoryWidgets/W_Inventory.W_Inventory_C|GetW_CraftingBenchWindow _w_inventory) CanCratf?))))

(event Custom|UpdateTribeMessage
  (params (MOTD :type Text))
  (Default|SetTribeMessage (Variables|/Game/_Main/Widgets/TribeWidgets/W_TribeSwitcher.W_TribeSwitcher_C|GetW_TribeWindow (Variables|/Game/_Main/Widgets/W_MainWidget.W_MainWidget_C|GetW_TribeSwitcher (Variables|Default|GetMainWidgetRef))) MOTD))

(event Custom|ShowCraftingProgressBar
  (Default|ShowCraftingBar (Variables|Default|GetMainWidgetRef)))

(event Custom|UpdateStatBar
  (params (Stat :type E_StatEnum%20Enum :default "NewEnumerator0") (Current :type Float%20%28double-precision%29) (Max :type Float%20%28double-precision%29))
  ;[1 1 1] Update Player Stats Widgets
  (Default|UpdateBar (Variables|/Game/_Main/Widgets/W_MainWidget.W_MainWidget_C|GetW_PlayerStatsWindow (Variables|Default|GetMainWidgetRef)) Stat Current Max)
  (Default|UpdateStat (Variables|/Game/_Main/Widgets/InventoryWidgets/W_Inventory.W_Inventory_C|GetW_PlayerInfoWindow (Variables|/Game/_Main/Widgets/W_MainWidget.W_MainWidget_C|GetW_Inventory (Variables|Default|GetMainWidgetRef))) Stat Current Max))

(event Custom|ShowOrHideDehydrated
  (params (ShowOrHide? :type Boolean))
  (bind _mainwidgetref (Variables|Default|GetMainWidgetRef))
  ;[1 1 1] Update Player Stats Widgets
  (if ShowOrHide?
    (Default|ShowDehydratedNotifi _mainwidgetref)
    (else
      (Default|RemoveDehydratedNotifi _mainwidgetref))))

(event Custom|ShowOrHideStarving
  (params (ShowOrHide? :type Boolean))
  (bind _mainwidgetref (Variables|Default|GetMainWidgetRef))
  ;[1 1 1] Update Player Stats Widgets
  (if ShowOrHide?
    (Default|ShowStarvingNotifi _mainwidgetref)
    (else
      (Default|RemoveStarvingNotifi _mainwidgetref))))

(event Custom|UpdateExperienceUI
  (params (CurrentExp :type Integer) (MaxExp :type Integer))
  ;[1 1 1] Experience and Level Notifications
  (Default|UpdateExperience (Variables|/Game/_Main/Widgets/InventoryWidgets/W_Inventory.W_Inventory_C|GetW_PlayerInfoWindow (Variables|/Game/_Main/Widgets/W_MainWidget.W_MainWidget_C|GetW_Inventory (Variables|Default|GetMainWidgetRef))) CurrentExp MaxExp))

(event EventBeginPlay
  (Networking|SwitchHasAuthority
    (:Remote
      (bind _returnvalue (UserInterface|CreateWidget "/Game/_Main/Widgets/W_MainWidget.W_MainWidget_C" self))
      (bind _output_get (Variables|Default|SetMainWidgetRef _returnvalue))
      (UserInterface|Viewport|AddtoViewport _output_get 0))))

(event Input|KeyboardEvents|Tab
  (params (Key :type Key%20Structure :default "None"))
  ;[0 0 0] Show / Hide Inventory
  (:Pressed
    (CallFunction|ShoworHideInventory)))

(event Input|KeyboardEvents|I
  (params (Key :type Key%20Structure :default "None"))
  ;[0 0 0] Show / Hide Inventory
  (:Pressed
    (CallFunction|ShoworHideInventory)))

(fn ConstructionScript)

(fn GetInventoryWidget
  (params (Container :type E_ContainerType%20Enum :default "NewEnumerator0") (SlotIndex :type Integer))
  (return (Utilities|Array|Get(acopy) (Variables|/Game/_Main/Widgets/InventoryWidgets/W_ItemContainerGrid.W_ItemContainerGrid_C|GetSlots (Utilities|Select :Index Container :NewEnumerator0 (Variables|/Game/_Main/Widgets/InventoryWidgets/W_Inventory.W_Inventory_C|GetW_ItemContainerGrid (Variables|/Game/_Main/Widgets/W_MainWidget.W_MainWidget_C|GetW_Inventory (Variables|Default|GetMainWidgetRef))) :NewEnumerator1 (Variables|/Game/_Main/Widgets/InventoryWidgets/W_HotBar.W_HotBar_C|GetW_ItemContainerGrid (Variables|/Game/_Main/Widgets/W_MainWidget.W_MainWidget_C|GetW_HotBar (Variables|Default|GetMainWidgetRef))) :NewEnumerator2 (Variables|/Game/_Main/Widgets/InventoryWidgets/W_Inventory.W_Inventory_C|GetStorageBoxGrid (Variables|/Game/_Main/Widgets/W_MainWidget.W_MainWidget_C|GetW_Inventory (Variables|Default|GetMainWidgetRef))) :NewEnumerator3 0)) SlotIndex)))

(fn CreateTribeFunction
  (params (TribeName :type Text))
  (bind _returnvalue (Math|DateTime|Now))
  (bind _self self)
  (bind _uniquenetid (Class|AdvancedSessionsLibrary|GetUniqueNetID _self))
  (bind (_year _month _day _hour _minute) (Math|DateTime|BreakDateTime _returnvalue))
  (bind _string (Class|AdvancedSessionsLibrary|UniqueNetIdtoString _uniquenetid))
  (LocalVariables|SetLocalTribeName TribeName)
  (bind _gamestateref (Class|BPISurvivalGameState|GetGameStateRef(Message) (Game|GetGameState)))
  (bind _playerstateref (Class|BPISurvivalPlayerState|GetPlayerStateRef(Message) (Variables|GetPlayerState)))
  (Variables|/Game/_Main/Blueprints/GameModes/SurvivalGame_PlayerState.SurvivalGame_PlayerState_C|SetTribeName _playerstateref (LocalVariables|GetLocalTribeName))
  (Variables|/Game/_Main/Blueprints/GameModes/SurvivalGame_PlayerState.SurvivalGame_PlayerState_C|SetTribeID _playerstateref _string)
  (LocalVariables|SetLocalTribeWindow (Utilities|Struct|MakeS_TribeInfo (LocalVariables|GetLocalTribeName) _string (Utilities|Array|MakeArray (Utilities|Struct|MakeS_TribeMemberInfo (Variables|/Game/_Main/Blueprints/GameModes/SurvivalGame_PlayerState.SurvivalGame_PlayerState_C|GetPlayerName _playerstateref) 0 true self "NewEnumerator0" (Class|AdvancedSessionsLibrary|UniqueNetIdtoString _uniquenetid))) "" (Utilities|Array|MakeArray (Utilities|Struct|MakeS_TribeLogEntry (Utilities|Text|FormatText "{Hour}:{Minute}" (Utilities|Text|ToText(Integer) _hour) (Utilities|Text|ToText(Integer) _minute)) (Utilities|Text|FormatText "{Mounth}/{Day}/{Year}" (Utilities|Text|ToText(Integer) _month) (Utilities|Text|ToText(Integer) _day) (Utilities|Text|ToText(Integer) _year)) (Utilities|Text|FormatText (Variables|/Game/_Main/Blueprints/GameModes/SurvivalGame_PlayerState.SurvivalGame_PlayerState_C|GetPlayerName _playerstateref)) "NewEnumerator2"))))
  (Default|CreateNewTribe _gamestateref (LocalVariables|GetLocalTribeWindow))
  (CallFunction|UpdateTribeWindow (LocalVariables|GetLocalTribeWindow))
  (Variables|/Game/_Main/Blueprints/GameModes/SurvivalGame_PlayerState.SurvivalGame_PlayerState_C|SetIsInTribe? _playerstateref true)
  (CallFunction|ShowTribeWindow)
  (CallFunction|UpdateTribeButtons "NewEnumerator0")
  (bind _survivalcharref (Class|BPISurvivalCharacter|GetSurvivalCharRef(Message) (Pawn|GetControlledPawn)))
  (Default|MergeTribeStructures _survivalcharref))

(fn JoinTribeFunction
  (params (TribeID :type String) (PlayerWhoInvited :type Text))
  (LocalVariables|SetLocalTribeID TribeID)
  (LocalVariables|SetLocalPlayerName PlayerWhoInvited)
  (bind _playerstateref (Class|BPISurvivalPlayerState|GetPlayerStateRef(Message) (Variables|GetPlayerState)))
  (if (not (Variables|/Game/_Main/Blueprints/GameModes/SurvivalGame_PlayerState.SurvivalGame_PlayerState_C|GetIsInTribe? _playerstateref))
    (Variables|/Game/_Main/Blueprints/GameModes/SurvivalGame_PlayerState.SurvivalGame_PlayerState_C|SetIsInTribe? _playerstateref true)
    (Variables|/Game/_Main/Blueprints/GameModes/SurvivalGame_PlayerState.SurvivalGame_PlayerState_C|SetTribeID _playerstateref (LocalVariables|GetLocalTribeID))
    (Variables|/Game/_Main/Blueprints/GameModes/SurvivalGame_PlayerState.SurvivalGame_PlayerState_C|SetTribeRank _playerstateref "NewEnumerator2")
    (bind _gamestateref (Class|BPISurvivalGameState|GetGameStateRef(Message) (Game|GetGameState)))
    (Default|AddTribeMember _gamestateref (LocalVariables|GetLocalTribeID) (Utilities|Struct|MakeS_TribeMemberInfo (Variables|/Game/_Main/Blueprints/GameModes/SurvivalGame_PlayerState.SurvivalGame_PlayerState_C|GetPlayerName _playerstateref) 0 true self "NewEnumerator2" (Class|AdvancedSessionsLibrary|UniqueNetIdtoString (Class|AdvancedSessionsLibrary|GetUniqueNetID self))) (LocalVariables|GetLocalPlayerName))
    (CallFunction|RemoveTribeInviteBox)
    (bind _tribeinfo (Class|BPISurvivalGameState|GetTribeInfo(Message) (Game|GetGameState) (LocalVariables|GetLocalTribeID)))
    (CallFunction|UpdateTribeWindow _tribeinfo)
    (CallFunction|ShowTribeWindow)
    (bind _playerstateref_2 (Class|BPISurvivalPlayerState|GetPlayerStateRef(Message) (Variables|GetPlayerState)))
    (Variables|/Game/_Main/Blueprints/GameModes/SurvivalGame_PlayerState.SurvivalGame_PlayerState_C|SetTribeName _playerstateref_2 (Utilities|Struct|BreakS_TribeInfo _tribeinfo))
    (CallFunction|UpdateTribeButtons "NewEnumerator2")))

(fn DemoteMemberFunction
  (params (MemberID :type String))
  (Networking|SwitchHasAuthority
    (:Authority
      (bind _playerstateref (Class|BPISurvivalPlayerState|GetPlayerStateRef(Message) (Variables|GetPlayerState)))
      (if (or (Utilities|Enum|Equal(Enum) (Variables|/Game/_Main/Blueprints/GameModes/SurvivalGame_PlayerState.SurvivalGame_PlayerState_C|GetTribeRank _playerstateref) "NewEnumerator0") (Utilities|Enum|Equal(Enum) (Variables|/Game/_Main/Blueprints/GameModes/SurvivalGame_PlayerState.SurvivalGame_PlayerState_C|GetTribeRank _playerstateref) "NewEnumerator1"))
        (bind _gamestateref (Class|BPISurvivalGameState|GetGameStateRef(Message) (Game|GetGameState)))
        (Default|DemoteTribeMember _gamestateref MemberID (Variables|/Game/_Main/Blueprints/GameModes/SurvivalGame_PlayerState.SurvivalGame_PlayerState_C|GetTribeID _playerstateref) (Variables|/Game/_Main/Blueprints/GameModes/SurvivalGame_PlayerState.SurvivalGame_PlayerState_C|GetPlayerName _playerstateref))))))

(fn PromoteMemberFunction
  (params (TribeMemberID :type String))
  (Networking|SwitchHasAuthority
    (:Authority
      (bind _playerstateref (Class|BPISurvivalPlayerState|GetPlayerStateRef(Message) (Variables|GetPlayerState)))
      (if (or (Utilities|Enum|Equal(Enum) (Variables|/Game/_Main/Blueprints/GameModes/SurvivalGame_PlayerState.SurvivalGame_PlayerState_C|GetTribeRank _playerstateref) "NewEnumerator0") (Utilities|Enum|Equal(Enum) (Variables|/Game/_Main/Blueprints/GameModes/SurvivalGame_PlayerState.SurvivalGame_PlayerState_C|GetTribeRank _playerstateref) "NewEnumerator1"))
        (bind _gamestateref (Class|BPISurvivalGameState|GetGameStateRef(Message) (Game|GetGameState)))
        (Default|PromoteTribeMember _gamestateref TribeMemberID (Variables|/Game/_Main/Blueprints/GameModes/SurvivalGame_PlayerState.SurvivalGame_PlayerState_C|GetTribeID _playerstateref) (Variables|/Game/_Main/Blueprints/GameModes/SurvivalGame_PlayerState.SurvivalGame_PlayerState_C|GetPlayerName _playerstateref))))))

(fn KickMemberFunction
  (params (TribeMemberID :type String))
  (Networking|SwitchHasAuthority
    (:Authority
      (bind _playerstateref (Class|BPISurvivalPlayerState|GetPlayerStateRef(Message) (Variables|GetPlayerState)))
      (if (or (Utilities|Enum|Equal(Enum) (Variables|/Game/_Main/Blueprints/GameModes/SurvivalGame_PlayerState.SurvivalGame_PlayerState_C|GetTribeRank _playerstateref) "NewEnumerator0") (Utilities|Enum|Equal(Enum) (Variables|/Game/_Main/Blueprints/GameModes/SurvivalGame_PlayerState.SurvivalGame_PlayerState_C|GetTribeRank _playerstateref) "NewEnumerator1"))
        (bind _gamestateref (Class|BPISurvivalGameState|GetGameStateRef(Message) (Game|GetGameState)))
        (Default|KickTribeMember _gamestateref TribeMemberID (Variables|/Game/_Main/Blueprints/GameModes/SurvivalGame_PlayerState.SurvivalGame_PlayerState_C|GetTribeID _playerstateref) (Variables|/Game/_Main/Blueprints/GameModes/SurvivalGame_PlayerState.SurvivalGame_PlayerState_C|GetPlayerName _playerstateref))))))

(fn LeaveTribeFunction
  (Networking|SwitchHasAuthority
    (:Authority
      (bind _playerstateref (Class|BPISurvivalPlayerState|GetPlayerStateRef(Message) (Variables|GetPlayerState)))
      (if (Utilities|Enum|NotEqual(Enum) (Variables|/Game/_Main/Blueprints/GameModes/SurvivalGame_PlayerState.SurvivalGame_PlayerState_C|GetTribeRank _playerstateref) "NewEnumerator0")
        (bind _gamestateref (Class|BPISurvivalGameState|GetGameStateRef(Message) (Game|GetGameState)))
        (Default|LeaveTribe _gamestateref (Variables|/Game/_Main/Blueprints/GameModes/SurvivalGame_PlayerState.SurvivalGame_PlayerState_C|GetTribeID _playerstateref) (Class|AdvancedSessionsLibrary|UniqueNetIdtoString (Class|AdvancedSessionsLibrary|GetUniqueNetID self)))
        (CallFunction|ResetTribeWindow)))))

(fn SurvivalLostPCRef
  (return self))