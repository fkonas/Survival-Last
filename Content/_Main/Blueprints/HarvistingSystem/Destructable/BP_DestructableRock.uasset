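; BP_DestructableRock is the destroyed-rock effect actor in the harvesting system, playing out a rock breaking apart and then removing itself.
; On BeginPlay it spawns a BP_DestructionForce at its location and calls MulticastFX, which plays the rock destruction particles and an attenuated sound there.
; After a fixed delay of a few seconds, the actor destroys itself.
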(event Custom|MulticastFX
  (bind _returnvalue (Transformation|GetActorLocation))
  (Effects|SpawnEmitteratLocation "/Game/Realistic_Starter_VFX_Pack_Vol2/Particles/Destruction/P_DestructionRock.P_DestructionRock" _returnvalue)
  (Audio|PlaySoundatLocation "/Game/_Main/Sounds/Harvesting/SC_RockDestroy.SC_RockDestroy" _returnvalue "0, 0, 0" 1.0 1.0 0.0 "/Game/_Main/Sounds/Harvesting/HarvestingAtt.HarvestingAtt" 0 0 0))

(event EventBeginPlay
  (Networking|SwitchHasAuthority
    (:Authority
      _)
    (:Remote
      _))
  (Game|SpawnActorfromClass "/Game/_Main/Blueprints/HarvistingSystem/Destructable/BP_DestructionForce.BP_DestructionForce_C" (Math|Transform|MakeTransform (Transformation|GetActorLocation) "0, 0, 0" "1.000000,1.000000,1.000000") "Undefined" 0 0)
  (CallFunction|MulticastFX)
  (Utilities|FlowControl|Delay 8.0)
  (Actor|DestroyActor))

(fn ConstructionScript
  (|CallParentFunction))