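; Player hotbar inventory component, a child of a shared container class, holding the items in the player's quick slots.
; Slot drops from inventory, hotbar or storage route through TransferItem.
; Add and remove overrides call the parent, then update the controller's slot display; removal also tells the survival character to dequip.
; DropItem spawns a BP_WorldItem at the character's arrow and clears the slot, always using index 0 rather than the passed index.
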(event EventBeginPlay)

(event EventTick
  (params (DeltaSeconds :type Float%20%28single-precision%29)))

(fn CheckHotbar
  (params (Index :type Integer))
  (bind _items (Variables|Default|GetItems))
  (bind _output (Utilities|Array|Get(acopy) _items Index))
  (bind (_itemid _itemquantity _itemicon _itemname _itemdescription _itemdamage _itemrarity _itemcurrenthp _itemmaxhp _isstackable_ _stacksize _itemtype) (Utilities|Struct|BreakS_ItemInfo _output))
  (if (== _itemid 0)
    (return false "NewEnumerator0")
    (else
      (return true _itemtype))))

(fn HandleSlotDrop
  (params (FromContainer :type BPC%20Item%20Container%20Object%20Reference) (FromIndex :type Integer) (DroppedIndex :type Integer))
  (LocalVariables|SetLocalFromContainer FromContainer)
  (LocalVariables|SetLocalFromIndex FromIndex)
  (LocalVariables|SetLocalDroppedIndex DroppedIndex)
  (switch Utilities|FlowControl|Switch|SwitchonE_ContainerType (Variables|/Game/_Main/Blueprints/Inventory/BPC_ItemContainer.BPC_ItemContainer_C|GetContainerType (LocalVariables|GetLocalFromContainer))
    (:NewEnumerator0
      _)
    (:NewEnumerator1
      _)
    (:NewEnumerator2
      _))
  (Default|TransferItem (LocalVariables|GetLocalFromContainer) self (LocalVariables|GetLocalDroppedIndex) (LocalVariables|GetLocalFromIndex))
  (return))

(fn AddItemtoIndex
  (params (Item :type S%20Item%20Info%20Structure) (LocalSpecificIndex :type Integer) (FromIndex :type Integer))
  (bind (_success_ _updatequantity_ _quantity) (|CallParentFunction Item LocalSpecificIndex FromIndex))
  (bind _controllerref (Class|BPISurvivalCharacter|GetControllerfromCharacter(Message) (Components|GetOwner)))
  (Default|UpdateItemSlot _controllerref (Variables|Default|GetContainerType) LocalSpecificIndex (CallFunction|GetItematIndex LocalSpecificIndex))
  (return _success_ _updatequantity_ _quantity))

(fn RemoveItematIndex
  (params (Index :type Integer))
  (bind _success_ (|CallParentFunction Index))
  (bind _controllerref (Class|BPISurvivalCharacter|GetControllerfromCharacter(Message) (Components|GetOwner)))
  (Default|ResetItemSlot _controllerref (Variables|Default|GetContainerType) Index)
  (bind _survivalcharref (Class|BPISurvivalCharacter|GetSurvivalCharRef(Message) (Components|GetOwner)))
  (Default|DequipCurrentItem _survivalcharref Index)
  (return _success_))

(fn DropItem
  (params (ItemIndex :type Integer))
  (LocalVariables|SetLocalItemIndex 0)
  (if (not (CallFunction|IsSlotEmpty? (LocalVariables|GetLocalItemIndex)))
    (bind _survivalcharref (Class|BPISurvivalCharacter|GetSurvivalCharRef(Message) (Components|GetOwner)))
    (Game|SpawnActorfromClass "/Game/_Main/Blueprints/Items/WorldItemBag/BP_WorldItem.BP_WorldItem_C" (Math|Transform|MakeTransform (Transformation|GetWorldLocation (Variables|/Game/_Main/Blueprints/Character/BP_FirstPersonMan.BP_FirstPersonMan_C|GetArrow1 _survivalcharref)) "0, 0, 0" "1.000000,1.000000,1.000000") "Undefined" 0 (Utilities|Array|Get(acopy) (Variables|Default|GetItems) (LocalVariables|GetLocalItemIndex)) 0)
    (CallFunction|RemoveItematIndex (LocalVariables|GetLocalItemIndex))))