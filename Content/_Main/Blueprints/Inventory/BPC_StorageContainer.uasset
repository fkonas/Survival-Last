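; Inventory component for storage containers and bags, extending a parent item container with storage-specific slot handling.
; Slot drops route TransferItem by source type, covering moves from player inventory, hotbar or within storage.
; Add and remove overrides call the parent, then update widgets through the owning storage actor; bags delete the array entry instead of resetting the slot.
; Dropping an item spawns BP_WorldItem at the owner's drop location and removes it from storage.
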(fn HandleSlotDrop
  (params (FromContainer :type BPC%20Item%20Container%20Object%20Reference) (FromIndex :type Integer) (DroppedIndex :type Integer))
  (LocalVariables|SetLocalFromContainer FromContainer)
  (LocalVariables|SetLocalFromIndex FromIndex)
  (LocalVariables|SetLocalDroppedIndex DroppedIndex)
  (switch Utilities|FlowControl|Switch|SwitchonE_ContainerType (Variables|/Game/_Main/Blueprints/Inventory/BPC_ItemContainer.BPC_ItemContainer_C|GetContainerType (LocalVariables|GetLocalFromContainer))
    (:NewEnumerator0
      _)
    (:NewEnumerator1
      _)
    (:NewEnumerator2
      (Default|TransferItem self self (LocalVariables|GetLocalDroppedIndex) (LocalVariables|GetLocalFromIndex))
      (return)))
  (Default|TransferItem (LocalVariables|GetLocalFromContainer) self (LocalVariables|GetLocalDroppedIndex) (LocalVariables|GetLocalFromIndex))
  (return))

(fn AddItemtoIndex
  (params (Item :type S%20Item%20Info%20Structure) (LocalSpecificIndex :type Integer) (FromIndex :type Integer))
  (LocalVariables|SetLocalIndex LocalSpecificIndex)
  (bind (_success_ _updatequantity_ _quantity) (|CallParentFunction Item LocalSpecificIndex FromIndex))
  (if _success_
    (bind _ref (Class|BPIStorageBuildable|GetStorageReference(Message) (Components|GetOwner)))
    (Default|UpdateWidgets _ref (Variables|Default|GetContainerType) (LocalVariables|GetLocalIndex) (Utilities|Array|Get(acopy) (Variables|Default|GetItems) (LocalVariables|GetLocalIndex)))
    (return _success_ _updatequantity_ _quantity)
    (else
      (return _success_ _updatequantity_ _quantity))))

(fn RemoveItematIndex
  (params (Index :type Integer))
  (LocalVariables|SetLocalIndex Index)
  (bind _success_ (|CallParentFunction Index))
  (if _success_
    (bind _ref (Class|BPIStorageBuildable|GetStorageReference(Message) (Components|GetOwner)))
    (if (Variables|/Game/_Main/Blueprints/BuildingSystem/PlaceableStructures/BP_StorageBuildable.BP_StorageBuildable_C|GetIsBag? _ref)
      (Utilities|Array|RemoveIndex (Variables|Default|GetItems) (LocalVariables|GetLocalIndex))
      (bind _ref_2 (Class|BPIStorageBuildable|GetStorageReference(Message) (Components|GetOwner)))
      (Default|UpdateStorageUI _ref_2)
      (else
        (bind _ref_3 (Class|BPIStorageBuildable|GetStorageReference(Message) (Components|GetOwner)))
        (Default|ResetItemSlot _ref_3 (Variables|Default|GetContainerType) (LocalVariables|GetLocalIndex))
        (return false)))))

(fn DropItem
  (params (ItemIndex :type Integer))
  (LocalVariables|SetLocalItemIndex ItemIndex)
  (if (not (CallFunction|IsSlotEmpty? (LocalVariables|GetLocalItemIndex)))
    (bind _ref (Class|BPIStorageBuildable|GetStorageReference(Message) (Components|GetOwner)))
    (Game|SpawnActorfromClass "/Game/_Main/Blueprints/Items/WorldItemBag/BP_WorldItem.BP_WorldItem_C" (Math|Transform|MakeTransform (Transformation|GetWorldLocation (Variables|/Game/_Main/Blueprints/BuildingSystem/PlaceableStructures/BP_StorageBuildable.BP_StorageBuildable_C|GetItemDropLocation _ref)) "0, 0, 0" "1.000000,1.000000,1.000000") "Undefined" 0 (Utilities|Array|Get(acopy) (Variables|Default|GetItems) (LocalVariables|GetLocalItemIndex)) 0)
    (CallFunction|RemoveItematIndex (LocalVariables|GetLocalItemIndex))))