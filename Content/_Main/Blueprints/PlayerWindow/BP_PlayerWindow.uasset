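; BP_PlayerWindow is a preview actor that mirrors the player's held item and worn armor for display in a UI window.
; InitializeWindow creates a render target for its SceneCapture2D, wraps it in a dynamic material and passes that to the controller.
; Equip events spawn and attach items by socket and armor per slot, using Master Pose so armor follows the body mesh.
; Dequip events destroy them, and the held item also drives EquippedState.
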(event Custom|InitializeWindow
  (params (ControllerRef :type Survival%20Lost%20PC%20Object%20Reference))
  ;[0 0 0] Setup Scene Capture 2D Widget
  (bind _returnvalue (Rendering|CreateRenderTarget2D 500 800 "RTF_RGBA16f"))
  (Variables|/Script/Engine.SceneCaptureComponent2D|SetTextureTarget (Variables|Default|GetSceneCaptureComponent2D) _returnvalue)
  (bind _returnvalue_2 (Rendering|Material|CreateDynamicMaterialInstance "/Game/_Main/Blueprints/PlayerWindow/M_PlayerMaterial.M_PlayerMaterial" "None" "None" :!class /Script/Engine.KismetMaterialLibrary))
  (Rendering|Material|SetTextureParameterValue _returnvalue_2 "Param" _returnvalue)
  (Utilities|IsValid ControllerRef
    (:Is%20Valid
      (Default|SetRenderMaterial ControllerRef _returnvalue_2))))

(event Custom|EquipItemEvent
  (params (Info :type S%20Equipable%20Info%20Structure))
  (bind (_socketname _animationstate _firstpersonequipclass) (Utilities|Struct|BreakS_EquipableInfo Info))
  ;[0 0 0] Equip Item For Player Window
  (Variables|Default|SetEquippedState _animationstate)
  (bind _returnvalue (Game|SpawnActorfromClass _firstpersonequipclass (Math|Transform|MakeTransform "0, 0, 0" "0, 0, 0" "1.000000,1.000000,1.000000") "Undefined" 0 0))
  (bind _output_get (Variables|Default|SetEquippedItemRef _returnvalue))
  (Transformation|AttachComponentToComponent _output_get (Variables|Default|GetSkeletalMesh) _socketname "SnapToTarget" "SnapToTarget" "SnapToTarget" true))

(event Custom|DequipItemEvent
  ;[0 0 0] Dequip Item Player Window
  (bind _equippeditemref (Variables|Default|GetEquippedItemRef)
    (:then
      (Actor|DestroyActor _equippeditemref)
      (Variables|Default|SetEquippedState "NewEnumerator5"))
    (:else)))

(event Custom|EquipArmor
  (params (ItemInfo :type S%20Item%20Info%20Structure))
  ;[0 0 0] Equip Armor To Player Window
  (CallFunction|EquipArmorFunction ItemInfo))

(event Custom|DequipArmor
  (params (ArmorSlot :type E_ArmorType%20Enum :default "NewEnumerator0"))
  ;[0 0 0] Dequip Armor Player Window
  (switch Utilities|FlowControl|Switch|SwitchonE_ArmorType ArmorSlot
    (:NewEnumerator0
      (bind _helmetslot (Variables|Default|GetHelmetSlot)
        (:then
          (Actor|DestroyActor _helmetslot))
        (:else)))
    (:NewEnumerator1
      (bind _chestslot (Variables|Default|GetChestSlot)
        (:then
          (Actor|DestroyActor _chestslot))
        (:else)))
    (:NewEnumerator2
      (bind _pantsslot (Variables|Default|GetPantsSlot)
        (:then
          (Actor|DestroyActor _pantsslot))
        (:else)))
    (:NewEnumerator3
      (bind _bootsslot (Variables|Default|GetBootsSlot)
        (:then
          (Actor|DestroyActor _bootsslot))
        (:else)))))

(fn ConstructionScript)

(fn EquipArmorFunction
  (params (Item%20Info :type S%20Item%20Info%20Structure))
  (bind (_itemclassref _armortype) (Utilities|Struct|BreakS_ItemInfo Item%20Info))
  (LocalVariables|SetLocalArmor _armortype)
  (bind _returnvalue (Game|SpawnActorfromClass _itemclassref (Math|Transform|MakeTransform "0, 0, 0" "0, 0, 0" "1.000000,1.000000,1.000000") "Undefined" 0 0))
  (switch Utilities|FlowControl|Switch|SwitchonE_ArmorType (LocalVariables|GetLocalArmor)
    (:NewEnumerator0
      (bind _output_get (Variables|Default|SetHelmetSlot _returnvalue)))
    (:NewEnumerator1
      (bind _output_get_2 (Variables|Default|SetChestSlot _returnvalue)))
    (:NewEnumerator2
      (bind _output_get_3 (Variables|Default|SetPantsSlot _returnvalue)))
    (:NewEnumerator3
      (bind _output_get_4 (Variables|Default|SetBootsSlot _returnvalue))))
  (Transformation|AttachComponentToComponent (Utilities|Select :Index (LocalVariables|GetLocalArmor) :NewEnumerator0 _output_get :NewEnumerator1 _output_get_2 :NewEnumerator2 _output_get_3 :NewEnumerator3 _output_get_4) (Variables|Default|GetSkeletalMesh) "None" "SnapToTarget" "SnapToTarget" "SnapToTarget" true)
  (bind _armorref (Class|BPIArmorItem|GetArmorRef(Message) (Utilities|Select :Index (LocalVariables|GetLocalArmor) :NewEnumerator0 _output_get :NewEnumerator1 _output_get_2 :NewEnumerator2 _output_get_3 :NewEnumerator3 _output_get_4)))
  (Class|SkinnedMeshComponent|SetMasterPoseComponent (Variables|/Game/_Main/Blueprints/Items/BP_ArmorMaster.BP_ArmorMaster_C|GetSkeletalMesh _armorref) (Variables|Default|GetSkeletalMesh) false))

(fn GetPlayerWindowRef
  (return self))