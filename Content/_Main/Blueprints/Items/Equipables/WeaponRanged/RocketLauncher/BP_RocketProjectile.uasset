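; Rocket launcher projectile that explodes on impact and deals radial damage to nearby actors.
; On hit, the server multicasts the explosion particles, sound and mesh hiding, then applies flat damage through a sphere overlap, crediting the owning character's controller.
; It leaves a debug sphere at the blast point and destroys itself after a short delay.
; A getter exposes the damage tiers it can affect.
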(event Custom|RocketHitMulticast
  (params (Location :type Vector))
  (Effects|SpawnEmitteratLocation "/Game/MilitaryWeapDark/FX/P_RocketLauncher_Explosion_01.P_RocketLauncher_Explosion_01" Location)
  (Audio|SpawnSoundatLocation "/Game/MilitaryWeapDark/Sound/RocketLauncher/RocketLauncher_Explosion_Cue.RocketLauncher_Explosion_Cue" Location "0, 0, 0" 1.0 1.0 0.0 "/Game/MilitaryWeapDark/Sound/Attenuation/Explosion_att.Explosion_att" 0)
  (Rendering|SetVisibility (Variables|Default|GetStaticMesh) false false))

(event Collision|EventHit
  (params (MyComp :type Primitive%20Component%20Object%20Reference) (Other :type Actor%20Object%20Reference) (OtherComp :type Primitive%20Component%20Object%20Reference) (bSelfMoved :type Boolean) (HitLocation :type Vector :default "0, 0, 0") (HitNormal :type Vector :default "0, 0, 0") (NormalImpulse :type Vector :default "0, 0, 0") (Hit :type Hit%20Result%20Structure%20%28by%20ref%29))
  (Networking|SwitchHasAuthority
    (:Authority
      (CallFunction|RocketHitMulticast HitLocation)
      (bind (_outactors _returnvalue) (Collision|SphereOverlapActors HitLocation 1e+02 (Utilities|Array|MakeArray "ObjectTypeQuery3" "ObjectTypeQuery8") 0 (Utilities|Array|MakeArray self)))
      (Rendering|Debug|DrawDebugSphere HitLocation 1e+02 12 "(R=1.000000,G=0.000000,B=0.038396,A=1.000000)" 15.0)
      (if _returnvalue
        (for _array_element _outactors
          (Game|Damage|ApplyDamage _array_element 5e+01 (Pawn|GetController (Variables|Default|GetCharRef)) self "/Script/Engine.DamageType"))
        (Utilities|FlowControl|Delay 1.0)
        (Actor|DestroyActor)
        (else
          (Utilities|FlowControl|Delay 1.0)
          (Actor|DestroyActor))))))

(fn ConstructionScript)

(fn GetCanDamage
  (return (Variables|Default|GetDamage%20Tiers)))