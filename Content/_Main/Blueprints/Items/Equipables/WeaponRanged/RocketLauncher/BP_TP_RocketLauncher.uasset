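; Third-person rocket launcher equipable that fires single-shot rockets and handles reloading from inventory ammo.
; Use checks state and hotbar ammo, then passes camera rotation through client/server-named events to spawn BP_RocketProjectile at the Arrow.
; Firing plays sound and animations on both this and the first-person launcher, empties ammo and applies durability.
; Reload requires an empty launcher and a rocket item; EndAnimation consumes it, refills the slot and updates UI.
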(event Custom|CameraOnClient
  (params (Target :type BP%20First%20Person%20Man%20Object%20Reference))
  ;[0 0 0] Get Client Camera Rotation For Spawning Rocket Projectile
  (CallFunction|FireRocketonServer (Transformation|GetWorldRotation (Variables|/Game/_Main/Blueprints/Character/BP_FirstPersonMan.BP_FirstPersonMan_C|GetFirstPersonCamera Target))))

(event Custom|FireRocketOnServer
  (params (Rotation :type Rotator))
  (bind _char_ref (Variables|Default|GetChar%20Ref))
  ;[0 0 0] Fire Rocket On Server, Play Animations & Subtract Ammo
  (Class|BPISurvivalCharacter|FirstPersonMontage(Message) _char_ref "/Game/_Main/Blueprints/Character/Man/Animations/FPRocketFire_Montage.FPRocketFire_Montage")
  (Class|BPISurvivalCharacter|ThirdPersonMontage(Message) _char_ref "/Game/_Main/Blueprints/Character/Man/Animations/FPRocketFire_Montage.FPRocketFire_Montage")
  (CallFunction|SpawnProjectileonServer Rotation)
  (CallFunction|MulticastProjectile _char_ref)
  (CallFunction|FireRocketonClient (Variables|Default|GetChar%20Ref))
  (CallFunction|SubtractAmmo)
  (Default|SetItemDura (Variables|Default|GetChar%20Ref) 2)
  (Variables|Default|SetIsFiring? false))

(event Custom|MulticastProjectile
  (params (CharRef :type BP%20First%20Person%20Man%20Object%20Reference))
  ;[0 0 0] Spawn Rocket Projectile, Play Sounds and Animations
  (Audio|SpawnSoundAttached "/Game/MilitaryWeapDark/Sound/RocketLauncher/RocketLauncherB_Fire_Cue.RocketLauncherB_Fire_Cue" (Variables|Default|GetRocketLauncherMesh) "None" "0, 0, 0" "0, 0, 0" "KeepRelativeOffset" false 1.0 1.0 0.0 "/Game/MilitaryWeapDark/Sound/Attenuation/WeaponShot_att.WeaponShot_att" 0)
  (Components|Animation|PlayAnimation (Variables|Default|GetRocketLauncherMesh) "/Game/MilitaryWeapDark/Weapons/Anims/Fire_RocketLauncher_W.Fire_RocketLauncher_W" false))

(event Custom|FireRocketOnClient
  (params (CharRef :type BP%20First%20Person%20Man%20Object%20Reference))
  ;[0 0 0] Play Animations For First Person Character
  (bind _asbp_fp_rocket_launcher (Utilities|Casting|CastToBP_FP_RocketLauncher (Variables|/Game/_Main/Blueprints/Character/BP_FirstPersonMan.BP_FirstPersonMan_C|GetFirstPersonEquipItem CharRef)))
  (Components|Animation|PlayAnimation (Variables|/Game/_Main/Blueprints/Items/Equipables/WeaponRanged/RocketLauncher/BP_FP_RocketLauncher.BP_FP_RocketLauncher_C|GetRocketLauncherMesh _asbp_fp_rocket_launcher) "/Game/MilitaryWeapDark/Weapons/Anims/Fire_RocketLauncher_W.Fire_RocketLauncher_W" false))

(event Custom|SpawnProjectileOnServer
  (params (SpawnRotation :type Rotator))
  ;[0 0 0] Spawn Rocket Projectile, Play Sounds and Animations
  (Game|SpawnActorfromClass "/Game/_Main/Blueprints/Items/Equipables/WeaponRanged/RocketLauncher/BP_RocketProjectile.BP_RocketProjectile_C" (Math|Transform|MakeTransform (Transformation|GetWorldLocation (Variables|Default|GetArrow)) SpawnRotation "1.000000,1.000000,1.000000") "Undefined" 0 (Variables|Default|GetChar%20Ref) 0))

(event EventReloadItemEvent
  (params (CharRef :type BP%20First%20Person%20Man%20Object%20Reference))
  ;[0 0 0] Rocket Reload Check
  (Variables|Default|SetChar%20Ref CharRef)
  (if (not (Variables|Default|GetIsReloading?))
    (bind _survivalcharref (Class|BPISurvivalCharacter|GetSurvivalCharRef(Message) CharRef))
    (if (<= (Utilities|Struct|BreakS_ItemInfo (Utilities|Array|Get(acopy) (Variables|/Game/_Main/Blueprints/Inventory/BPC_ItemContainer.BPC_ItemContainer_C|GetItems (Variables|/Game/_Main/Blueprints/Character/BP_FirstPersonMan.BP_FirstPersonMan_C|GetBPC_PlayerHotBar _survivalcharref)) (Variables|/Game/_Main/Blueprints/Character/BP_FirstPersonMan.BP_FirstPersonMan_C|GetHotbarIndex _survivalcharref))) 0)
      (bind _survivalcharref_2 (Class|BPISurvivalCharacter|GetSurvivalCharRef(Message) (Variables|Default|GetChar%20Ref)))
      (bind (_index _iteminfo _hasitem_) (Default|FindItem (Variables|/Game/_Main/Blueprints/Character/BP_FirstPersonMan.BP_FirstPersonMan_C|GetBPC_PlayerInventory _survivalcharref_2) 77))
      (if _hasitem_
        (Variables|Default|SetAmmoIndex _index)
        (Variables|Default|SetIsReloading? true)
        (Class|BPISurvivalCharacter|FirstPersonMontage(Message) (Variables|Default|GetChar%20Ref) "/Game/_Main/Blueprints/Character/Man/Animations/FPRocketReload_Montage.FPRocketReload_Montage")
        (Class|BPISurvivalCharacter|ThirdPersonMontage(Message) (Variables|Default|GetChar%20Ref) "/Game/_Main/Blueprints/Character/Man/Animations/FPRocketReload_Montage.FPRocketReload_Montage")))))

(event EventEndAnimation
  ;[0 0 0] Remove Ammo From Inventory, Update Weapon Slot UI
  (if (Variables|Default|GetIsReloading?)
    (bind _survivalcharref (Class|BPISurvivalCharacter|GetSurvivalCharRef(Message) (Variables|Default|GetChar%20Ref)))
    (Default|RemoveQuantity (Variables|/Game/_Main/Blueprints/Character/BP_FirstPersonMan.BP_FirstPersonMan_C|GetBPC_PlayerInventory _survivalcharref) (Variables|Default|GetAmmoIndex) 1)
    (bind _structout (Utilities|Struct|SetmembersinS_ItemInfo (Utilities|Array|Get(acopy) (Variables|/Game/_Main/Blueprints/Inventory/BPC_ItemContainer.BPC_ItemContainer_C|GetItems (Variables|/Game/_Main/Blueprints/Character/BP_FirstPersonMan.BP_FirstPersonMan_C|GetBPC_PlayerHotBar _survivalcharref)) (Variables|/Game/_Main/Blueprints/Character/BP_FirstPersonMan.BP_FirstPersonMan_C|GetHotbarIndex _survivalcharref)) 1))
    (Utilities|Array|SetArrayElem (Variables|/Game/_Main/Blueprints/Inventory/BPC_ItemContainer.BPC_ItemContainer_C|GetItems (Variables|/Game/_Main/Blueprints/Character/BP_FirstPersonMan.BP_FirstPersonMan_C|GetBPC_PlayerHotBar _survivalcharref)) (Variables|/Game/_Main/Blueprints/Character/BP_FirstPersonMan.BP_FirstPersonMan_C|GetHotbarIndex _survivalcharref) _structout)
    (bind _controllerref (Class|BPISurvivalCharacter|GetControllerfromCharacter(Message) (Variables|Default|GetChar%20Ref)))
    (Default|UpdateItemSlot _controllerref "NewEnumerator1" (Variables|/Game/_Main/Blueprints/Character/BP_FirstPersonMan.BP_FirstPersonMan_C|GetHotbarIndex _survivalcharref) _structout)
    (Variables|Default|SetIsReloading? false)))

(event EventUseItemInterface
  (params (CharRef :type BP%20First%20Person%20Man%20Object%20Reference))
  ;[0 0 0] Do Checks to see if we can fire rocket launcher
  (bind _output_get (Variables|Default|SetChar%20Ref CharRef))
  (if (not (Variables|Default|GetIsFiring?))
    (if (not (Variables|Default|GetIsReloading?))
      (if (>= (Utilities|Struct|BreakS_ItemInfo (Utilities|Array|Get(acopy) (Variables|/Game/_Main/Blueprints/Inventory/BPC_ItemContainer.BPC_ItemContainer_C|GetItems (Variables|/Game/_Main/Blueprints/Character/BP_FirstPersonMan.BP_FirstPersonMan_C|GetBPC_PlayerHotBar _output_get)) (Variables|/Game/_Main/Blueprints/Character/BP_FirstPersonMan.BP_FirstPersonMan_C|GetHotbarIndex _output_get))) 1)
        (Variables|Default|SetIsFiring? true)
        (CallFunction|CameraonClient (Variables|Default|GetChar%20Ref))))))

(fn ConstructionScript
  (|CallParentFunction))

(fn SubtractAmmo
  (bind _survivalcharref (Class|BPISurvivalCharacter|GetSurvivalCharRef(Message) (Variables|Default|GetChar%20Ref)))
  (bind _structout (Utilities|Struct|SetmembersinS_ItemInfo (Utilities|Array|Get(acopy) (Variables|/Game/_Main/Blueprints/Inventory/BPC_ItemContainer.BPC_ItemContainer_C|GetItems (Variables|/Game/_Main/Blueprints/Character/BP_FirstPersonMan.BP_FirstPersonMan_C|GetBPC_PlayerHotBar _survivalcharref)) (Variables|/Game/_Main/Blueprints/Character/BP_FirstPersonMan.BP_FirstPersonMan_C|GetHotbarIndex _survivalcharref))))
  (Utilities|Array|SetArrayElem (Variables|/Game/_Main/Blueprints/Inventory/BPC_ItemContainer.BPC_ItemContainer_C|GetItems (Variables|/Game/_Main/Blueprints/Character/BP_FirstPersonMan.BP_FirstPersonMan_C|GetBPC_PlayerHotBar _survivalcharref)) (Variables|/Game/_Main/Blueprints/Character/BP_FirstPersonMan.BP_FirstPersonMan_C|GetHotbarIndex _survivalcharref) _structout)
  (bind _controllerref (Class|BPISurvivalCharacter|GetControllerfromCharacter(Message) (Variables|Default|GetChar%20Ref)))
  (Default|UpdateItemSlot _controllerref "NewEnumerator1" (Variables|/Game/_Main/Blueprints/Character/BP_FirstPersonMan.BP_FirstPersonMan_C|GetHotbarIndex _survivalcharref) _structout))