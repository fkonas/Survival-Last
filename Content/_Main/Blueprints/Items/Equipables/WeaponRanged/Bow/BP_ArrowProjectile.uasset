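; Bow arrow projectile that sticks into Damageable actors and deals location-based damage.
; Only the first hit counts: the arrow attaches, overlaps pawns, then runs a complex forward trace on the Camera channel to find the surface struck.
; Players take damage scaled by physical-material body zone and reduced by armor in that slot, sent through a message call.
; Other Damageable actors receive boosted point damage.
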(event Collision|EventHit
  (params (MyComp :type Primitive%20Component%20Object%20Reference) (Other :type Actor%20Object%20Reference) (OtherComp :type Primitive%20Component%20Object%20Reference) (bSelfMoved :type Boolean) (HitLocation :type Vector :default "0, 0, 0") (HitNormal :type Vector :default "0, 0, 0") (NormalImpulse :type Vector :default "0, 0, 0") (Hit :type Hit%20Result%20Structure%20%28by%20ref%29))
  (Utilities|FlowControl|DoOnce false
    (:Completed
      (if (Actor|ActorHasTag Other "Damageable")
        (Transformation|AttachActorToActor self Other "None" "KeepWorld" "KeepWorld" "KeepWorld" true)
        (Collision|SetCollisionResponsetoChannel (Variables|Default|GetSphere) "ECC_Pawn" "ECR_Overlap")
        (Variables|Default|SetArrowLocation (Transformation|GetWorldLocation (Variables|Default|GetArrowMesh)))
        (bind (_outhit _returnvalue) (Collision|LineTraceByChannel (Variables|Default|GetArrowLocation) (+ (Variables|Default|GetArrowLocation) (* (Transformation|GetActorForwardVector) (Variables|Default|GetTraceDistance))) "TraceTypeQuery2" true (Utilities|Array|MakeArray self) "ForDuration"))
        (if _returnvalue
          (if (Actor|ActorHasTag (.HitActor (Collision|BreakHitResult _outhit)) "Damageable")
            (CallFunction|ApllyDamages (.HitActor (Collision|BreakHitResult _outhit)) _outhit (Variables|/Script/PhysicsCore.PhysicalMaterial|GetSurfaceType (.PhysMat (Collision|BreakHitResult _outhit))))))))))

(fn ConstructionScript)

(fn ApllyDamages
  (params (DamageActor :type Actor%20Object%20Reference) (HitInfo :type Hit%20Result%20Structure) (SurfaceHit :type EPhysicalSurface%20Enum :default "SurfaceType_Default"))
  (LocalVariables|SetPSurfaceHit SurfaceHit)
  (LocalVariables|SetLocalDamage (* (Variables|Default|GetItemDamage) (LocalVariables|GetDamageMultipler)))
  (if (Actor|ActorHasTag DamageActor "player")
    (LocalVariables|SetLocalDamage (Utilities|Select :Index (LocalVariables|GetPSurfaceHit) :SurfaceType_Default (* (LocalVariables|GetLocalDamage) 1.0) :SurfaceType1 (* (LocalVariables|GetLocalDamage) 8.0) :SurfaceType2 (* (LocalVariables|GetLocalDamage) 5.0) :SurfaceType3 (* (LocalVariables|GetLocalDamage) 3.0) :SurfaceType4 (* (LocalVariables|GetLocalDamage) 1.0) :SurfaceType5 (* (LocalVariables|GetLocalDamage) 1.0)))
    (bind _hasarmor_ (Class|BPISurvivalCharacter|HasArmorinSlot?(Message) DamageActor (LocalVariables|GetPSurfaceHit)))
    (if _hasarmor_
      (LocalVariables|SetLocalDamage (- (LocalVariables|GetLocalDamage) (* (LocalVariables|GetLocalDamage) 0.25))))
    (Class|BPISurvivalCharacter|WeaponRangedDamage(Message) DamageActor (LocalVariables|GetLocalDamage) 0 self (LocalVariables|GetPSurfaceHit))
    (Development|PrintString (Utilities|String|ToString(Float) (LocalVariables|GetLocalDamage)))
    (else
      (Game|Damage|ApplyPointDamage DamageActor (* (LocalVariables|GetLocalDamage) 4.0) (Variables|Default|GetArrowLocation) HitInfo 0 self "/Script/Engine.DamageType"))))