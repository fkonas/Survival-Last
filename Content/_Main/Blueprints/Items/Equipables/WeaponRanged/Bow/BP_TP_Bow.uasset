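; Third-person bow equipable that handles drawing, reloading and firing arrows for a survival character.
; Use draws a loaded bow, or first moves an arrow from inventory into hotbar ammo after a short delay.
; Releasing left mouse sends camera rotation to the server, which clears ammo, spawns BP_ArrowProjectile and applies durability.
; Multicast events animate this mesh and toggle its arrow, while client events mirror them on BP_FP_Bow.
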(event Custom|DrawBowOnClient
  (params (CharRef :type BP%20First%20Person%20Man%20Object%20Reference))
  ;[0 0 0] Draw Bow on Client an Multicast
  (bind _asbp_fp_bow (Utilities|Casting|CastToBP_FP_Bow (Variables|/Game/_Main/Blueprints/Character/BP_FirstPersonMan.BP_FirstPersonMan_C|GetFirstPersonEquipItem CharRef)))
  (Components|Animation|PlayAnimation (Variables|/Game/_Main/Blueprints/Items/Equipables/WeaponRanged/Bow/BP_FP_Bow.BP_FP_Bow_C|GetBowMesh _asbp_fp_bow) "/Game/_Main/Meshes/Equipables/Bow/BowAnim.BowAnim" false)
  (Default|HideArrow _asbp_fp_bow true))

(event Custom|MulticastDrawBow
  ;[0 0 0] Draw Bow on Client an Multicast
  (Components|Animation|PlayAnimation (Variables|Default|GetBowMesh) "/Game/_Main/Meshes/Equipables/Bow/BowAnim.BowAnim" false)
  (Rendering|SetVisibility (Variables|Default|GetArrowMesh) true false))

(event Custom|CameraOnClient
  (params (Target :type BP%20First%20Person%20Man%20Object%20Reference))
  ;[0 0 0] Fire Bow On Server
  (CallFunction|FireBowonServer (Transformation|GetWorldRotation (Variables|/Game/_Main/Blueprints/Character/BP_FirstPersonMan.BP_FirstPersonMan_C|GetFirstPersonCamera Target))))

(event Custom|FireBowOnServer
  (params (Rotation :type Rotator))
  (bind _char_ref (Variables|Default|GetChar%20Ref))
  ;[0 0 0] Fire Bow On Server
  (bind _survivalcharref (Class|BPISurvivalCharacter|GetSurvivalCharRef(Message) (Variables|Default|GetChar%20Ref)))
  (bind _structout (Utilities|Struct|SetmembersinS_ItemInfo (Utilities|Array|Get(acopy) (Variables|/Game/_Main/Blueprints/Inventory/BPC_ItemContainer.BPC_ItemContainer_C|GetItems (Variables|/Game/_Main/Blueprints/Character/BP_FirstPersonMan.BP_FirstPersonMan_C|GetBPC_PlayerHotBar _survivalcharref)) (Variables|/Game/_Main/Blueprints/Character/BP_FirstPersonMan.BP_FirstPersonMan_C|GetHotbarIndex _survivalcharref))))
  (Utilities|Array|SetArrayElem (Variables|/Game/_Main/Blueprints/Inventory/BPC_ItemContainer.BPC_ItemContainer_C|GetItems (Variables|/Game/_Main/Blueprints/Character/BP_FirstPersonMan.BP_FirstPersonMan_C|GetBPC_PlayerHotBar _survivalcharref)) (Variables|/Game/_Main/Blueprints/Character/BP_FirstPersonMan.BP_FirstPersonMan_C|GetHotbarIndex _survivalcharref) _structout)
  (bind _controllerref (Default|GetControllerfromCharacter (Variables|Default|GetChar%20Ref)))
  (Default|UpdateItemSlot _controllerref "NewEnumerator1" (Variables|/Game/_Main/Blueprints/Character/BP_FirstPersonMan.BP_FirstPersonMan_C|GetHotbarIndex _survivalcharref) _structout)
  (Class|BPISurvivalCharacter|FirstPersonMontage(Message) _char_ref "/Game/_Main/Blueprints/Character/Man/Animations/Bow_Shoot_Montage.Bow_Shoot_Montage")
  (Class|BPISurvivalCharacter|ThirdPersonMontage(Message) _char_ref "/Game/_Main/Blueprints/Character/Man/Animations/Bow_Shoot_Montage.Bow_Shoot_Montage")
  (Game|SpawnActorfromClass "/Game/_Main/Blueprints/Items/Equipables/WeaponRanged/Bow/BP_ArrowProjectile.BP_ArrowProjectile_C" (Math|Transform|MakeTransform (Transformation|GetWorldLocation (Variables|/Game/_Main/Blueprints/Character/BP_FirstPersonMan.BP_FirstPersonMan_C|GetArrow1 (Variables|Default|GetChar%20Ref))) Rotation "1.000000,1.000000,1.000000") "Undefined" 0 (Variables|Default|GetChar%20Ref) 0)
  (CallFunction|FireBowMulticast)
  (CallFunction|FireBowonClient (Variables|Default|GetChar%20Ref))
  (Default|SetItemDura (Variables|Default|GetChar%20Ref) 1)
  (Variables|Default|SetIsFiring? false))

(event Custom|FireBowMulticast
  ;[0 0 0] Fire Bow Mulitcast and Client Events
  (Components|Animation|PlayAnimation (Variables|Default|GetBowMesh) 0 false)
  (Rendering|SetVisibility (Variables|Default|GetArrowMesh) false false))

(event Custom|FireBowOnClient
  (params (CharRef :type BP%20First%20Person%20Man%20Object%20Reference))
  ;[0 0 0] Fire Bow Mulitcast and Client Events
  (bind _asbp_fp_bow (Utilities|Casting|CastToBP_FP_Bow (Variables|/Game/_Main/Blueprints/Character/BP_FirstPersonMan.BP_FirstPersonMan_C|GetFirstPersonEquipItem CharRef)))
  (Components|Animation|PlayAnimation (Variables|/Game/_Main/Blueprints/Items/Equipables/WeaponRanged/Bow/BP_FP_Bow.BP_FP_Bow_C|GetBowMesh _asbp_fp_bow) 0 false)
  (Default|HideArrow _asbp_fp_bow false))

(event Custom|ReloadArrow
  ;[1 1 1] Reload Bow Logic
  (if (not (Variables|Default|GetIsReloading?))
    (bind _survivalcharref (Class|BPISurvivalCharacter|GetSurvivalCharRef(Message) (Variables|Default|GetChar%20Ref)))
    (if (<= (Utilities|Struct|BreakS_ItemInfo (Utilities|Array|Get(acopy) (Variables|/Game/_Main/Blueprints/Inventory/BPC_ItemContainer.BPC_ItemContainer_C|GetItems (Variables|/Game/_Main/Blueprints/Character/BP_FirstPersonMan.BP_FirstPersonMan_C|GetBPC_PlayerHotBar _survivalcharref)) (Variables|/Game/_Main/Blueprints/Character/BP_FirstPersonMan.BP_FirstPersonMan_C|GetHotbarIndex _survivalcharref))) 0)
      (bind _survivalcharref_2 (Class|BPISurvivalCharacter|GetSurvivalCharRef(Message) (Variables|Default|GetChar%20Ref)))
      (bind (_index _iteminfo _hasitem_) (Default|FindItem (Variables|/Game/_Main/Blueprints/Character/BP_FirstPersonMan.BP_FirstPersonMan_C|GetBPC_PlayerInventory _survivalcharref_2) 79))
      (if _hasitem_
        (Variables|Default|SetAmmoIndex _index)
        (Variables|Default|SetIsReloading? true)
        (if (Variables|Default|GetIsReloading?)
          (bind _survivalcharref_3 (Class|BPISurvivalCharacter|GetSurvivalCharRef(Message) (Variables|Default|GetChar%20Ref)))
          (Default|RemoveQuantity (Variables|/Game/_Main/Blueprints/Character/BP_FirstPersonMan.BP_FirstPersonMan_C|GetBPC_PlayerInventory _survivalcharref_3) (Variables|Default|GetAmmoIndex) 1)
          (bind _structout (Utilities|Struct|SetmembersinS_ItemInfo (Utilities|Array|Get(acopy) (Variables|/Game/_Main/Blueprints/Inventory/BPC_ItemContainer.BPC_ItemContainer_C|GetItems (Variables|/Game/_Main/Blueprints/Character/BP_FirstPersonMan.BP_FirstPersonMan_C|GetBPC_PlayerHotBar _survivalcharref_3)) (Variables|/Game/_Main/Blueprints/Character/BP_FirstPersonMan.BP_FirstPersonMan_C|GetHotbarIndex _survivalcharref_3)) 1))
          (Utilities|Array|SetArrayElem (Variables|/Game/_Main/Blueprints/Inventory/BPC_ItemContainer.BPC_ItemContainer_C|GetItems (Variables|/Game/_Main/Blueprints/Character/BP_FirstPersonMan.BP_FirstPersonMan_C|GetBPC_PlayerHotBar _survivalcharref_3)) (Variables|/Game/_Main/Blueprints/Character/BP_FirstPersonMan.BP_FirstPersonMan_C|GetHotbarIndex _survivalcharref_3) _structout)
          (Utilities|FlowControl|Delay 1.0)
          (bind _controllerref (Class|BPISurvivalCharacter|GetControllerfromCharacter(Message) (Variables|Default|GetChar%20Ref)))
          (Default|UpdateItemSlot _controllerref "NewEnumerator1" (Variables|/Game/_Main/Blueprints/Character/BP_FirstPersonMan.BP_FirstPersonMan_C|GetHotbarIndex _survivalcharref_3) _structout)
          (Variables|Default|SetIsReloading? false)
          (CallFunction|DrawBow))))))

(event Custom|DrawBow
  (bind _char_ref (Variables|Default|GetChar%20Ref))
  (bind _char_ref_2 (Variables|Default|GetChar%20Ref))
  ;[0 0 0] Conduct Checks to Fire Bow, And Play Draw Back Animations
  (if (>= (Utilities|Struct|BreakS_ItemInfo (Utilities|Array|Get(acopy) (Variables|/Game/_Main/Blueprints/Inventory/BPC_ItemContainer.BPC_ItemContainer_C|GetItems (Variables|/Game/_Main/Blueprints/Character/BP_FirstPersonMan.BP_FirstPersonMan_C|GetBPC_PlayerHotBar _char_ref)) (Variables|/Game/_Main/Blueprints/Character/BP_FirstPersonMan.BP_FirstPersonMan_C|GetHotbarIndex _char_ref))) 1)
    (Variables|Default|SetIsFiring? true)
    (CallFunction|DrawBowonClient _char_ref_2)
    (Class|BPISurvivalCharacter|FirstPersonMontage(Message) _char_ref_2 "/Game/_Main/Blueprints/Character/Man/Animations/Bow_Draw_Montage.Bow_Draw_Montage")
    (Class|BPISurvivalCharacter|ThirdPersonMontage(Message) _char_ref_2 "/Game/_Main/Blueprints/Character/Man/Animations/Bow_Draw_Montage.Bow_Draw_Montage")
    (CallFunction|MulticastDrawBow)))

(event EventStopLeftMouseLoop
  (if (Variables|Default|GetIsFiring?)
    (CallFunction|CameraonClient (Variables|Default|GetChar%20Ref))))

(event EventUseItemInterface
  (params (CharRef :type BP%20First%20Person%20Man%20Object%20Reference))
  ;[0 0 0] Conduct Checks to Fire Bow, And Play Draw Back Animations
  (bind _output_get (Variables|Default|SetChar%20Ref CharRef))
  (if (not (Variables|Default|GetIsFiring?))
    (if (not (Variables|Default|GetIsReloading?))
      (if (>= (Utilities|Struct|BreakS_ItemInfo (Utilities|Array|Get(acopy) (Variables|/Game/_Main/Blueprints/Inventory/BPC_ItemContainer.BPC_ItemContainer_C|GetItems (Variables|/Game/_Main/Blueprints/Character/BP_FirstPersonMan.BP_FirstPersonMan_C|GetBPC_PlayerHotBar _output_get)) (Variables|/Game/_Main/Blueprints/Character/BP_FirstPersonMan.BP_FirstPersonMan_C|GetHotbarIndex _output_get))) 1)
        (Variables|Default|SetIsFiring? true)
        (CallFunction|DrawBowonClient (Variables|Default|GetChar%20Ref))
        (Class|BPISurvivalCharacter|FirstPersonMontage(Message) (Variables|Default|GetChar%20Ref) "/Game/_Main/Blueprints/Character/Man/Animations/Bow_Draw_Montage.Bow_Draw_Montage")
        (Class|BPISurvivalCharacter|ThirdPersonMontage(Message) (Variables|Default|GetChar%20Ref) "/Game/_Main/Blueprints/Character/Man/Animations/Bow_Draw_Montage.Bow_Draw_Montage")
        (CallFunction|MulticastDrawBow)
        (else
          (CallFunction|ReloadArrow))))))

(fn ConstructionScript
  (|CallParentFunction))