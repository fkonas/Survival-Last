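; Third-person rifle item for a survival game, handling automatic fire, hit damage and reloading.
; Holding left click loops a timer that passes camera rotation to FireRifleOnServer, which plays montages and effects, line traces and decrements hotbar ammo.
; Player damage scales by hit physical surface and armor, while other damageable actors take multiplied generic damage.
; Reload finds inventory ammo, then updates inventory and hotbar slot when EndAnimation fires.
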(event Custom|StartFire
  ;[0 0 0] Start Fire Loop
  (bind _returnvalue (Utilities|Time|SetTimerbyEvent (delegate Custom|FireEvent) 0.2 true))
  (Variables|Default|SetRifleFireTimer _returnvalue))

(event Custom|FireEvent
  ;[0 0 0] Start Fire Loop
  (bind _survivalcharref (Class|BPISurvivalCharacter|GetSurvivalCharRef(Message) (Variables|Default|GetChar%20Ref)))
  (if (>= (Utilities|Struct|BreakS_ItemInfo (Utilities|Array|Get(acopy) (Variables|/Game/_Main/Blueprints/Inventory/BPC_ItemContainer.BPC_ItemContainer_C|GetItems (Variables|/Game/_Main/Blueprints/Character/BP_FirstPersonMan.BP_FirstPersonMan_C|GetBPC_PlayerHotBar _survivalcharref)) (Variables|/Game/_Main/Blueprints/Character/BP_FirstPersonMan.BP_FirstPersonMan_C|GetHotbarIndex _survivalcharref))) 1)
    (CallFunction|GetCameraRotation (Variables|Default|GetChar%20Ref))))

(event Custom|GetCameraRotation
  (params (Target :type BP%20First%20Person%20Man%20Object%20Reference))
  ;[0 0 0] Get Camera Rotation for Line Trace
  (CallFunction|FireRifleonServer (Transformation|GetWorldRotation (Variables|/Game/_Main/Blueprints/Character/BP_FirstPersonMan.BP_FirstPersonMan_C|GetFirstPersonCamera Target))))

(event Custom|FireRifleOnServer
  (params (Rotation :type Rotator))
  (bind _char_ref (Variables|Default|GetChar%20Ref))
  ;[0 0 0] Fire Rifle Events, Line Trace and Apply Damage
  (Variables|Default|SetPlayerCameraRot Rotation)
  (Class|BPISurvivalCharacter|FirstPersonMontage(Message) _char_ref "/Game/_Main/Blueprints/Character/Man/Animations/FPRifleIdleFire_Montage.FPRifleIdleFire_Montage")
  (Class|BPISurvivalCharacter|ThirdPersonMontage(Message) _char_ref "/Game/_Main/Blueprints/Character/Man/Animations/FPRifleIdleFire_Montage.FPRifleIdleFire_Montage")
  (CallFunction|MulticastFire)
  (CallFunction|RifleFireFirstPerson (Variables|Default|GetChar%20Ref))
  (bind (_outhit _hit_) (CallFunction|LineTrace (Variables|Default|GetPlayerCameraRot)))
  (if _hit_
    (CallFunction|ApplyDamages (.HitActor (Collision|BreakHitResult _outhit)) _outhit (Actor|ActorHasTag (.HitActor (Collision|BreakHitResult _outhit)) "Damageable") (Variables|/Script/PhysicsCore.PhysicalMaterial|GetSurfaceType (.PhysMat (Collision|BreakHitResult _outhit)))))
  (CallFunction|SubtractAmmo))

(event Custom|MulticastFire
  (bind _rifle (Variables|Default|GetRifle))
  ;[0 0 0] Play Rifle Fire FX and Sound for all neabry players
  (Components|Animation|PlayAnimation _rifle "/Game/MilitaryWeapDark/Weapons/Anims/Fire_Rifle_W.Fire_Rifle_W" false)
  (Audio|SpawnSoundAttached "/Game/MilitaryWeapDark/Sound/Rifle/RifleB_Fire_Cue.RifleB_Fire_Cue" _rifle "None" "0, 0, 0" "0, 0, 0" "KeepRelativeOffset" false 1.0 1.0 0.0 "/Game/MilitaryWeapDark/Sound/Attenuation/WeaponShot_att.WeaponShot_att" 0))

(event Custom|RifleFireFirstPerson
  (params (Char :type BP%20First%20Person%20Man%20Object%20Reference))
  ;[0 0 0] Play Rifle Fire FX For First Person View
  (bind _asbp_fp_rifle (Utilities|Casting|CastToBP_FP_Rifle (Variables|/Game/_Main/Blueprints/Character/BP_FirstPersonMan.BP_FirstPersonMan_C|GetFirstPersonEquipItem Char)))
  (Components|Animation|PlayAnimation (Variables|/Game/_Main/Blueprints/Items/Equipables/WeaponRanged/Rifle/BP_FP_Rifle.BP_FP_Rifle_C|GetRifle _asbp_fp_rifle) "/Game/MilitaryWeapDark/Weapons/Anims/Fire_Rifle_W.Fire_Rifle_W" false))

(event Custom|ReloadWeaponOnClient
  (params (Char :type BP%20First%20Person%20Man%20Object%20Reference))
  ;[0 0 0] Play Reload Animation on Rifle for First Person Mode
  (bind _asbp_fp_rifle (Utilities|Casting|CastToBP_FP_Rifle (Variables|/Game/_Main/Blueprints/Character/BP_FirstPersonMan.BP_FirstPersonMan_C|GetFirstPersonEquipItem Char)))
  (Components|Animation|PlayAnimation (Variables|/Game/_Main/Blueprints/Items/Equipables/WeaponRanged/Rifle/BP_FP_Rifle.BP_FP_Rifle_C|GetRifle _asbp_fp_rifle) "/Game/MilitaryWeapDark/Weapons/Anims/Reload_Rifle_Hip_W.Reload_Rifle_Hip_W" false))

(event EventReloadItemEvent
  (params (CharRef :type BP%20First%20Person%20Man%20Object%20Reference))
  (bind _char_ref (Variables|Default|GetChar%20Ref))
  ;[0 0 0] Reload Checks, If we can reload our rifle, if we ave enough ammo, and play animations
  (if (not (Variables|Default|GetIsReloading?))
    (bind _survivalcharref (Class|BPISurvivalCharacter|GetSurvivalCharRef(Message) CharRef))
    (if (< (.CurrentAmmo (Utilities|Struct|BreakS_ItemInfo (Utilities|Array|Get(acopy) (Variables|/Game/_Main/Blueprints/Inventory/BPC_ItemContainer.BPC_ItemContainer_C|GetItems (Variables|/Game/_Main/Blueprints/Character/BP_FirstPersonMan.BP_FirstPersonMan_C|GetBPC_PlayerHotBar _survivalcharref)) (Variables|/Game/_Main/Blueprints/Character/BP_FirstPersonMan.BP_FirstPersonMan_C|GetHotbarIndex _survivalcharref)))) (.MaxAmmo (Utilities|Struct|BreakS_ItemInfo (Utilities|Array|Get(acopy) (Variables|/Game/_Main/Blueprints/Inventory/BPC_ItemContainer.BPC_ItemContainer_C|GetItems (Variables|/Game/_Main/Blueprints/Character/BP_FirstPersonMan.BP_FirstPersonMan_C|GetBPC_PlayerHotBar _survivalcharref)) (Variables|/Game/_Main/Blueprints/Character/BP_FirstPersonMan.BP_FirstPersonMan_C|GetHotbarIndex _survivalcharref)))))
      (Variables|Default|SetCurrent%20Ammo (.CurrentAmmo (Utilities|Struct|BreakS_ItemInfo (Utilities|Array|Get(acopy) (Variables|/Game/_Main/Blueprints/Inventory/BPC_ItemContainer.BPC_ItemContainer_C|GetItems (Variables|/Game/_Main/Blueprints/Character/BP_FirstPersonMan.BP_FirstPersonMan_C|GetBPC_PlayerHotBar _survivalcharref)) (Variables|/Game/_Main/Blueprints/Character/BP_FirstPersonMan.BP_FirstPersonMan_C|GetHotbarIndex _survivalcharref)))))
      (bind _char_ref_2 (Variables|Default|GetChar%20Ref)
        (:then
          (bind _survivalcharref_2 (Class|BPISurvivalCharacter|GetSurvivalCharRef(Message) _char_ref_2))
          (bind (_index _iteminfo _hasitem_) (Default|FindItem (Variables|/Game/_Main/Blueprints/Character/BP_FirstPersonMan.BP_FirstPersonMan_C|GetBPC_PlayerInventory _survivalcharref_2) 75))
          (if _hasitem_
            (Variables|Default|SetAmmoIndex _index)
            (Variables|Default|SetTotalAmmo (Utilities|Struct|BreakS_ItemInfo _iteminfo))
            (Variables|Default|SetIsReloading? true)
            (Class|BPISurvivalCharacter|FirstPersonMontage(Message) _char_ref "/Game/_Main/Blueprints/Character/Man/Animations/RifleReload_Montage.RifleReload_Montage")
            (Class|BPISurvivalCharacter|ThirdPersonMontage(Message) _char_ref "/Game/_Main/Blueprints/Character/Man/Animations/RifleReload_Montage.RifleReload_Montage")
            (CallFunction|ReloadWeapononClient (Variables|Default|GetChar%20Ref))))
        (:else)))))

(event EventEndAnimation
  ;[0 0 0] Reload Animations After are Played
  (if (Variables|Default|GetIsReloading?)
    (bind _survivalcharref (Class|BPISurvivalCharacter|GetSurvivalCharRef(Message) (Variables|Default|GetChar%20Ref)))
    (Variables|Default|SetTempAmmo (Variables|Default|GetCurrent%20Ammo))
    (Variables|Default|SetCurrent%20Ammo (Math|Integer|SelectInt (Variables|Default|GetMaxClipSize) (+ (Variables|Default|GetCurrent%20Ammo) (Variables|Default|GetTotalAmmo)) (>= (+ (Variables|Default|GetCurrent%20Ammo) (Variables|Default|GetTotalAmmo)) (Variables|Default|GetMaxClipSize))))
    (Variables|Default|SetAmmoToRemove (Math|Integer|Clamp(Integer) (Math|Integer|SelectInt (- (Variables|Default|GetMaxClipSize) (Variables|Default|GetTempAmmo)) (Variables|Default|GetMaxClipSize) (>= (+ (Variables|Default|GetCurrent%20Ammo) (Variables|Default|GetTotalAmmo)) (Variables|Default|GetMaxClipSize))) 0 (Variables|Default|GetTotalAmmo)))
    (bind (_removed_ _removedamount) (Default|RemoveQuantity (Variables|/Game/_Main/Blueprints/Character/BP_FirstPersonMan.BP_FirstPersonMan_C|GetBPC_PlayerInventory _survivalcharref) (Variables|Default|GetAmmoIndex) (Variables|Default|GetAmmoToRemove)))
    (bind _structout (Utilities|Struct|SetmembersinS_ItemInfo (Utilities|Array|Get(acopy) (Variables|/Game/_Main/Blueprints/Inventory/BPC_ItemContainer.BPC_ItemContainer_C|GetItems (Variables|/Game/_Main/Blueprints/Character/BP_FirstPersonMan.BP_FirstPersonMan_C|GetBPC_PlayerHotBar _survivalcharref)) (Variables|/Game/_Main/Blueprints/Character/BP_FirstPersonMan.BP_FirstPersonMan_C|GetHotbarIndex _survivalcharref)) (select _removed_ _removedamount (Variables|Default|GetCurrent%20Ammo))))
    (Utilities|Array|SetArrayElem (Variables|/Game/_Main/Blueprints/Inventory/BPC_ItemContainer.BPC_ItemContainer_C|GetItems (Variables|/Game/_Main/Blueprints/Character/BP_FirstPersonMan.BP_FirstPersonMan_C|GetBPC_PlayerHotBar _survivalcharref)) (Variables|/Game/_Main/Blueprints/Character/BP_FirstPersonMan.BP_FirstPersonMan_C|GetHotbarIndex _survivalcharref) _structout)
    (bind _controllerref (Class|BPISurvivalCharacter|GetControllerfromCharacter(Message) (Variables|Default|GetChar%20Ref)))
    (Default|UpdateItemSlot _controllerref "NewEnumerator1" (Variables|/Game/_Main/Blueprints/Character/BP_FirstPersonMan.BP_FirstPersonMan_C|GetHotbarIndex _survivalcharref) _structout)
    (Variables|Default|SetIsReloading? false)
    (Default|SetItemDura (Variables|Default|GetChar%20Ref) 1)))

(event EventUseItemInterface
  (params (CharRef :type BP%20First%20Person%20Man%20Object%20Reference))
  ;[0 0 0] Use Item Event LeftClick
  (bind _output_get (Variables|Default|SetChar%20Ref CharRef))
  (if (not (Variables|Default|GetIsReloading?))
    (if (>= (Utilities|Struct|BreakS_ItemInfo (Utilities|Array|Get(acopy) (Variables|/Game/_Main/Blueprints/Inventory/BPC_ItemContainer.BPC_ItemContainer_C|GetItems (Variables|/Game/_Main/Blueprints/Character/BP_FirstPersonMan.BP_FirstPersonMan_C|GetBPC_PlayerHotBar _output_get)) (Variables|/Game/_Main/Blueprints/Character/BP_FirstPersonMan.BP_FirstPersonMan_C|GetHotbarIndex _output_get))) 1)
      (CallFunction|StartFire))))

(event EventStopLeftMouseLoop
  (Utilities|Time|ClearandInvalidateTimerbyHandle (Variables|Default|GetRifleFireTimer)))

(fn ConstructionScript
  (|CallParentFunction))

(fn LineTrace
  (params (PlayerCamera :type Rotator))
  (LocalVariables|SetCameraLocation (Transformation|GetWorldLocation (Variables|/Game/_Main/Blueprints/Character/BP_FirstPersonMan.BP_FirstPersonMan_C|GetFirstPersonCamera (Variables|Default|GetChar%20Ref))))
  (bind (_outhit _returnvalue) (Collision|LineTraceByChannel (LocalVariables|GetCameraLocation) (+ (LocalVariables|GetCameraLocation) (* (Math|Vector|GetForwardVector PlayerCamera) (Variables|Default|GetBulletDistance))) "TraceTypeQuery2" false (Utilities|Array|MakeArray self (Variables|Default|GetChar%20Ref)) "ForDuration"))
  (return _outhit _returnvalue))

(fn ApplyDamages
  (params (DamagedActor :type Actor%20Object%20Reference) (HitInfo :type Hit%20Result%20Structure) (Condition :type Boolean) (SurfaceHit :type EPhysicalSurface%20Enum :default "SurfaceType_Default"))
  (bind _output_get (LocalVariables|SetPSurfaceHit SurfaceHit))
  (Development|PrintString (Utilities|String|EnumtoString _output_get))
  (if Condition
    (LocalVariables|SetLocalDamage (* (Math|Conversions|ToFloat(Integer) (Utilities|Struct|BreakS_ItemInfo (Variables|Default|GetItemInfo))) (LocalVariables|GetDamageMultiplayer)))
    (if (Actor|ActorHasTag DamagedActor "player")
      ;[1 0.01661 0 0] Apply Different Damage Based On Hit Location
      (LocalVariables|SetLocalDamage (Utilities|Select :Index (LocalVariables|GetPSurfaceHit) :SurfaceType_Default (* (LocalVariables|GetLocalDamage) 1.0) :SurfaceType1 (* (LocalVariables|GetLocalDamage) 8.0) :SurfaceType2 (* (LocalVariables|GetLocalDamage) 5.0) :SurfaceType3 (* (LocalVariables|GetLocalDamage) 3.0) :SurfaceType4 (* (LocalVariables|GetLocalDamage) 1.0) :SurfaceType5 (* (LocalVariables|GetLocalDamage) 1.0)))
      ;[0 0 0] Calculate Damage Reduction Based on if Armor Equiped in Slot
      (bind _hasarmor_ (Class|BPISurvivalCharacter|HasArmorinSlot?(Message) DamagedActor (LocalVariables|GetPSurfaceHit)))
      (if _hasarmor_
        (LocalVariables|SetLocalDamage (- (LocalVariables|GetLocalDamage) (* (LocalVariables|GetLocalDamage) 0.25))))
      (Class|BPISurvivalCharacter|WeaponRangedDamage(Message) DamagedActor (LocalVariables|GetLocalDamage) (Pawn|GetController (Variables|Default|GetChar%20Ref)) self (LocalVariables|GetPSurfaceHit))
      (Development|PrintString (Utilities|String|ToString(Float) (LocalVariables|GetLocalDamage)))
      (else
        ;[0 0 0] Apply Damage to AI or Anything Other Than Player
        (Game|Damage|ApplyDamage DamagedActor (* (LocalVariables|GetLocalDamage) 4.0) (Pawn|GetController (Variables|Default|GetChar%20Ref)) self "/Script/Engine.DamageType")))))

(fn SubtractAmmo
  (bind _survivalcharref (Default|GetSurvivalCharRef (Variables|Default|GetChar%20Ref)))
  (bind _structout (Utilities|Struct|SetmembersinS_ItemInfo (Utilities|Array|Get(acopy) (Variables|/Game/_Main/Blueprints/Inventory/BPC_ItemContainer.BPC_ItemContainer_C|GetItems (Variables|/Game/_Main/Blueprints/Character/BP_FirstPersonMan.BP_FirstPersonMan_C|GetBPC_PlayerHotBar _survivalcharref)) (Variables|/Game/_Main/Blueprints/Character/BP_FirstPersonMan.BP_FirstPersonMan_C|GetHotbarIndex _survivalcharref)) (- (Utilities|Struct|BreakS_ItemInfo (Utilities|Array|Get(acopy) (Variables|/Game/_Main/Blueprints/Inventory/BPC_ItemContainer.BPC_ItemContainer_C|GetItems (Variables|/Game/_Main/Blueprints/Character/BP_FirstPersonMan.BP_FirstPersonMan_C|GetBPC_PlayerHotBar _survivalcharref)) (Variables|/Game/_Main/Blueprints/Character/BP_FirstPersonMan.BP_FirstPersonMan_C|GetHotbarIndex _survivalcharref))) 1)))
  (Utilities|Array|SetArrayElem (Variables|/Game/_Main/Blueprints/Inventory/BPC_ItemContainer.BPC_ItemContainer_C|GetItems (Variables|/Game/_Main/Blueprints/Character/BP_FirstPersonMan.BP_FirstPersonMan_C|GetBPC_PlayerHotBar _survivalcharref)) (Variables|/Game/_Main/Blueprints/Character/BP_FirstPersonMan.BP_FirstPersonMan_C|GetHotbarIndex _survivalcharref) _structout)
  (bind _controllerref (Default|GetControllerfromCharacter (Variables|Default|GetChar%20Ref)))
  (Default|UpdateItemSlot _controllerref "NewEnumerator1" (Variables|/Game/_Main/Blueprints/Character/BP_FirstPersonMan.BP_FirstPersonMan_C|GetHotbarIndex _survivalcharref) _structout))