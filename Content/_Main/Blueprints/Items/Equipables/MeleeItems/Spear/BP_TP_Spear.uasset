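; Equipable spear melee item that plays a jab montage on use and blocks re-use until the animation ends.
; An animation notify reads the owner's arrow location and passes it to ServerOverlap, which sphere-overlaps pawns there, ignoring the wielder.
; A hit updates item durability and damages each pawn found.
; Damage scales item base damage by a multiplier, reduced for player-tagged targets according to armor pieces worn.
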(event Custom|GetRotationOnClient
  ;[0 0 0] Get Camera Rotation/Location
  (bind _location (Class|BPISurvivalCharacter|GetArrowLocation(Message) (Components|GetOwner)))
  (CallFunction|ServerOverlap _location))

(event Custom|ServerOverlap
  (params (SpherePos :type Vector))
  ;[0 0 0] Sphere overlap, If Hit apply damage to pawn
  (bind (_outactors _returnvalue) (Collision|SphereOverlapActors SpherePos 6e+01 (Utilities|Array|MakeArray "ObjectTypeQuery3") 0 (Utilities|Array|MakeArray (Variables|Default|GetChar%20Ref))))
  (if _returnvalue
    (Default|SetItemDura (Variables|Default|GetChar%20Ref) 1)
    (for _array_element _outactors
      (bind _damage (CallFunction|CalculateDamage _array_element (Math|Conversions|ToFloat(Integer) (Utilities|Struct|BreakS_ItemInfo (Variables|Default|GetItemInfo)))))
      (Game|Damage|ApplyDamage _array_element _damage 0 self "/Script/Engine.DamageType"))))

(event EventUseItemInterface
  (params (CharRef :type BP%20First%20Person%20Man%20Object%20Reference))
  ;[0 0 0] Play Animation Montages
  (if (not (Variables|Default|GetIsSwinging?))
    (Variables|Default|SetIsSwinging? true)
    (bind _output_get (Variables|Default|SetChar%20Ref CharRef))
    (Class|BPISurvivalCharacter|FirstPersonMontage(Message) _output_get "/Game/_Main/Blueprints/Character/Man/Animations/FPSpearJab_Montage.FPSpearJab_Montage")
    (Class|BPISurvivalCharacter|ThirdPersonMontage(Message) _output_get "/Game/_Main/Blueprints/Character/Man/Animations/FPSpearJab_Montage.FPSpearJab_Montage")))

(event EventNotifyInterface
  ;[0 0 0] Get Camera Rotation/Location
  (CallFunction|GetRotationonClient))

(event EventEndAnimation
  ;[0 0 0] End Attack
  (Variables|Default|SetIsSwinging? false))

(fn ConstructionScript
  (|CallParentFunction))

(fn CalculateDamage
  (params (HitActor :type Actor%20Object%20Reference) (ItemBaseDamage :type Float%20%28double-precision%29))
  (LocalVariables|SetLocalDamage (* ItemBaseDamage (LocalVariables|GetDamageMultipler)))
  (if (Actor|ActorHasTag HitActor "player")
    (bind _totalarmorslots (Class|BPISurvivalCharacter|GetTotalArmorPieces(Message) HitActor))
    (switch int _totalarmorslots
      (:0
        (return (* (LocalVariables|GetLocalDamage) 4.0)))
      (:1
        (return (* (LocalVariables|GetLocalDamage) 3.5)))
      (:2
        (return (* (LocalVariables|GetLocalDamage) 3.0)))
      (:3
        (return (* (LocalVariables|GetLocalDamage) 2.5)))
      (:4
        (return (* (LocalVariables|GetLocalDamage) 2.0))))
    (else
      (return (* (LocalVariables|GetLocalDamage) 4.0)))))