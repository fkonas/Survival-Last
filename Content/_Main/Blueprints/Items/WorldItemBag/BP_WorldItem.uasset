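; BP_WorldItem is a world item bag that holds one item's info and gives it to the player who picks it up.
; PickupEvent runs once, adds BagItemInfo to the character's inventory component through AddItemOnServer, has the player controller show an item widget, then destroys the bag.
; On BeginPlay, the authority starts a three-minute timer that destroys the bag.
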(event Custom|DespawnBag
  (Actor|DestroyActor))

(event EventPickupEvent
  (params (CharRef :type BP%20First%20Person%20Man%20Object%20Reference) (Controller :type Controller%20Object%20Reference))
  (bind _bagiteminfo (Variables|Default|GetBagItemInfo))
  (bind (_itemquantity _itemicon _itemname) (Utilities|Struct|BreakS_ItemInfo _bagiteminfo))
  (Utilities|FlowControl|DoOnce false
    (:Completed
      (bind _survivalcharref (Class|BPISurvivalCharacter|GetSurvivalCharRef(Message) CharRef))
      (Default|AddItemonServer (Variables|/Game/_Main/Blueprints/Character/BP_FirstPersonMan.BP_FirstPersonMan_C|GetBPC_PlayerInventory _survivalcharref) (Variables|Default|GetBagItemInfo))
      (bind _playercontrollerref (Class|BPISurvivalLostPC|SurvivalLostPCRef(Message) Controller))
      (Default|ShowItemWidget _playercontrollerref _itemicon _itemquantity _itemname)
      (Actor|DestroyActor))))

(event EventBeginPlay
  (Networking|SwitchHasAuthority
    (:Authority
      (Utilities|Time|SetTimerbyEvent (delegate Custom|DespawnBag) 1.8e+02))))

(fn ConstructionScript)