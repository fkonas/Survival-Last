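; Game State for the survival game that holds all tribes in TribeMap and handles creation, membership, ranks, message of the day and log.
; Events call functions that edit copies of tribe structs, then assign TribeMap a new single-entry map holding that tribe.
; Changes append log entries and are pushed to online members' controllers for UI updates.
; Kick and leave share one function, which skips members of the first rank enumerator.
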(event Custom|CreateNewTribe
  (params (TribeInfo :type S%20Tribe%20Info%20Structure))
  (Utilities|Map|Add (Variables|Default|GetTribeMap) (Utilities|Struct|BreakS_TribeInfo TribeInfo) TribeInfo))

(event Custom|AddTribeMember
  (params (TribeID :type String) (MemberInfo :type S%20Tribe%20Member%20Info%20Structure) (PlayerWhoInitiated :type Text))
  (CallFunction|AddMember TribeID MemberInfo PlayerWhoInitiated))

(event Custom|AddTribeLogEvent
  (params (TribeID :type String) (TribeLogEvent :type S%20Tribe%20Log%20Entry%20Structure))
  (CallFunction|PosttoLog TribeID TribeLogEvent))

(event Custom|DemoteTribeMember
  (params (MemberID :type String) (TribeID :type String) (PlayerWhoInitiated :type Text))
  (CallFunction|DemoteTribeMemberFunction MemberID TribeID PlayerWhoInitiated))

(event Custom|PromoteTribeMember
  (params (TribeMemberID :type String) (TribeID :type String) (PlayerWhoInitiated :type Text))
  (CallFunction|PromoteTribeMemberFunction TribeMemberID TribeID PlayerWhoInitiated))

(event Custom|KickTribeMember
  (params (TribeMemberID :type String) (TribeID :type String) (PlayerWhoInitiated :type Text))
  (CallFunction|KickTribeMemberFunction TribeMemberID TribeID PlayerWhoInitiated))

(event Custom|LeaveTribe
  (params (TribeID :type String) (MemberID :type String))
  (CallFunction|LeaveTribeFunction MemberID TribeID false))

(event Custom|SetMOTD
  (params (TribeID :type String) (MOTD :type Text) (PlayerWhoInitiated :type Text))
  (CallFunction|TribeMessageOftheDay TribeID MOTD PlayerWhoInitiated))

(fn ConstructionScript)

(fn AddMember
  (params (TribeID :type String) (MemberInfo :type S%20Tribe%20Member%20Info%20Structure) (PlayerWhoInitiated :type Text))
  (LocalVariables|SetLocalTribeID TribeID)
  (LocalVariables|SetLocalMemberInfo MemberInfo)
  (LocalVariables|SetLocalPlayerName PlayerWhoInitiated)
  (if (.ReturnValue (Utilities|Map|Find (Variables|Default|GetTribeMap) (LocalVariables|GetLocalTribeID)))
    (LocalVariables|SetLocalMembers (Utilities|Struct|BreakS_TribeInfo (.Value (Utilities|Map|Find (Variables|Default|GetTribeMap) (LocalVariables|GetLocalTribeID)))))
    (Utilities|Array|Add (LocalVariables|GetLocalMembers) (LocalVariables|GetLocalMemberInfo))
    (bind _structout (Utilities|Struct|SetmembersinS_TribeInfo (.Value (Utilities|Map|Find (Variables|Default|GetTribeMap) (LocalVariables|GetLocalTribeID))) (LocalVariables|GetLocalMembers)))
    (|SetBy-RefVar (Variables|Default|GetTribeMap) (Utilities|Map|MakeMap (LocalVariables|GetLocalTribeID) _structout))
    (LocalVariables|SetLocalLogEvent (Utilities|Struct|MakeS_TribeLogEntry (Utilities|Text|ToText(Float) (Actor|GetGameTimeSinceCreation) "HalfToEven") "1" (Utilities|Text|FormatText "{PlayerWhoInvited} Added {Player} to the tribe!" (LocalVariables|GetLocalPlayerName) (Utilities|Struct|BreakS_TribeMemberInfo (LocalVariables|GetLocalMemberInfo))) "NewEnumerator2"))
    (CallFunction|UpdateMembersandLog (LocalVariables|GetLocalMembers) (LocalVariables|GetLocalLogEvent) (LocalVariables|GetLocalTribeID) true)))

(fn UpdateMembersandLog
  (params (MemberArray :type Array%20of%20S%20Tribe%20Member%20Info%20Structures) (LogEvent :type S%20Tribe%20Log%20Entry%20Structure) (TribeID :type String) (LogEvent? :type Boolean))
  (LocalVariables|SetLocalMembers MemberArray)
  (LocalVariables|SetLocalLogEvent LogEvent)
  (LocalVariables|SetLocalTribeID TribeID)
  (LocalVariables|SetLogEventLocal? LogEvent?)
  (CallFunction|AddLogtoArray (LocalVariables|GetLocalTribeID) (LocalVariables|GetLocalLogEvent))
  (for _array_element (LocalVariables|GetLocalMembers)
    (if (.IsOnline? (Utilities|Struct|BreakS_TribeMemberInfo _array_element))
      (Utilities|IsValid (.ControllerRef (Utilities|Struct|BreakS_TribeMemberInfo _array_element))
        (:Is%20Valid
          (Default|UpdateTribeMemmbers (.ControllerRef (Utilities|Struct|BreakS_TribeMemberInfo _array_element)) (LocalVariables|GetLocalMembers))
          (if (LocalVariables|GetLogEventLocal?)
            (Default|UpdateTribeLogUI (.ControllerRef (Utilities|Struct|BreakS_TribeMemberInfo _array_element)) (LocalVariables|GetLocalLogEvent))))))))

(fn AddLogtoArray
  (params (TribeID :type String) (LogToAdd :type S%20Tribe%20Log%20Entry%20Structure))
  (LocalVariables|SetLocalTribeID TribeID)
  (LocalVariables|SetLocalLogEvent LogToAdd)
  (LocalVariables|SetLocalLog (Utilities|Struct|BreakS_TribeInfo (.Value (Utilities|Map|Find (Variables|Default|GetTribeMap) (LocalVariables|GetLocalTribeID)))))
  (Utilities|Array|Add (LocalVariables|GetLocalLog) (LocalVariables|GetLocalLogEvent))
  (bind _structout (Utilities|Struct|SetmembersinS_TribeInfo (.Value (Utilities|Map|Find (Variables|Default|GetTribeMap) (LocalVariables|GetLocalTribeID))) (LocalVariables|GetLocalLog)))
  (|SetBy-RefVar (Variables|Default|GetTribeMap) (Utilities|Map|MakeMap (LocalVariables|GetLocalTribeID) _structout)))

(fn PosttoLog
  (params (TribeID :type String) (TribeLogEvent :type S%20Tribe%20Log%20Entry%20Structure))
  (bind _returnvalue (Math|DateTime|Now))
  (bind (_year _month _day _hour _minute) (Math|DateTime|BreakDateTime _returnvalue))
  (LocalVariables|SetLocalTribeID TribeID)
  (LocalVariables|SetTribeLogInfo TribeLogEvent)
  (bind _structout (Utilities|Struct|SetmembersinS_TribeLogEntry (LocalVariables|GetTribeLogInfo) (Utilities|Text|FormatText "{Hour}:{Minute}" (Utilities|Text|ToText(Integer) _hour) (Utilities|Text|ToText(Integer) _minute)) (Utilities|Text|FormatText "{Mounth}/{Day}/{Year}" (Utilities|Text|ToText(Integer) _month) (Utilities|Text|ToText(Integer) _day) (Utilities|Text|ToText(Integer) _year))))
  (LocalVariables|SetTribeLogInfo _structout)
  (CallFunction|AddLogtoArray (LocalVariables|GetLocalTribeID) (LocalVariables|GetTribeLogInfo))
  (if (.ReturnValue (Utilities|Map|Find (Variables|Default|GetTribeMap) (LocalVariables|GetLocalTribeID)))
    (LocalVariables|SetLocalMembers (Utilities|Struct|BreakS_TribeInfo (.Value (Utilities|Map|Find (Variables|Default|GetTribeMap) (LocalVariables|GetLocalTribeID)))))
    (for _array_element (LocalVariables|GetLocalMembers)
      (if (.IsOnline? (Utilities|Struct|BreakS_TribeMemberInfo _array_element))
        (Utilities|IsValid (.ControllerRef (Utilities|Struct|BreakS_TribeMemberInfo _array_element))
          (:Is%20Valid
            (Default|UpdateTribeLogUI (.ControllerRef (Utilities|Struct|BreakS_TribeMemberInfo _array_element)) (LocalVariables|GetTribeLogInfo))))))))

(fn DemoteTribeMemberFunction
  (params (MemberID :type String) (TribeID :type String) (PlayerWhoInitiated :type Text))
  (LocalVariables|SetLocalMemberID MemberID)
  (LocalVariables|SetLocalTribeID TribeID)
  (LocalVariables|SetLocalPlayerName PlayerWhoInitiated)
  (if (.ReturnValue (Utilities|Map|Find (Variables|Default|GetTribeMap) (LocalVariables|GetLocalTribeID)))
    (LocalVariables|SetLocalMembers (Utilities|Struct|BreakS_TribeInfo (.Value (Utilities|Map|Find (Variables|Default|GetTribeMap) (LocalVariables|GetLocalTribeID)))))
    (bind (_array_element _array_index) (Utilities|Array|ForEachLoopwithBreak (LocalVariables|GetLocalMembers) :!label _label)
      (:LoopBody
        (if (Utilities|Enum|Equal(Enum) (.PlayerIdOffline (Utilities|Struct|BreakS_TribeMemberInfo _array_element)) (LocalVariables|GetLocalMemberID))
          (LocalVariables|SetLocalIndex _array_index)
          (LocalVariables|SetLocalFound? true)
          (goto _label Break)))
      (:Completed
        (if (LocalVariables|GetLocalFound?)
          (bind _structout (Utilities|Struct|SetmembersinS_TribeMemberInfo (Utilities|Array|Get(acopy) (LocalVariables|GetLocalMembers) (LocalVariables|GetLocalIndex)) "NewEnumerator2"))
          (bind _output_get (LocalVariables|SetLocalMemberInfo _structout))
          (Utilities|Array|SetArrayElem (LocalVariables|GetLocalMembers) (LocalVariables|GetLocalIndex) _output_get)
          (bind _structout_2 (Utilities|Struct|SetmembersinS_TribeInfo (.Value (Utilities|Map|Find (Variables|Default|GetTribeMap) (LocalVariables|GetLocalTribeID))) (LocalVariables|GetLocalMembers)))
          (|SetBy-RefVar (Variables|Default|GetTribeMap) (Utilities|Map|MakeMap (LocalVariables|GetLocalTribeID) _structout_2))
          (Utilities|IsValid (.ControllerRef (Utilities|Struct|BreakS_TribeMemberInfo (LocalVariables|GetLocalMemberInfo)))
            (:Is%20Valid
              (Default|UpdateTribeRank (.ControllerRef (Utilities|Struct|BreakS_TribeMemberInfo (LocalVariables|GetLocalMemberInfo))) (.TribeRank (Utilities|Struct|BreakS_TribeMemberInfo (LocalVariables|GetLocalMemberInfo)))))
            (:Is%20Not%20Valid
              _))
          (LocalVariables|SetTribeLogEvent (Utilities|Struct|MakeS_TribeLogEntry (Utilities|Text|ToText(Float) (Actor|GetGameTimeSinceCreation) "HalfToEven") "1" (Utilities|Text|FormatText "{Initiator} Demoted {player} to {Rank}!" (LocalVariables|GetLocalPlayerName) (.PlayerName (Utilities|Struct|BreakS_TribeMemberInfo (LocalVariables|GetLocalMemberInfo))) (Utilities|Text|ToText(String) (Utilities|String|ToString(Byte) (.TribeRank (Utilities|Struct|BreakS_TribeMemberInfo (LocalVariables|GetLocalMemberInfo)))))) "NewEnumerator1"))
          (CallFunction|UpdateMembersandLog (LocalVariables|GetLocalMembers) (LocalVariables|GetTribeLogEvent) (LocalVariables|GetLocalTribeID) true))))))

(fn PromoteTribeMemberFunction
  (params (MemberID :type String) (TribeID :type String) (PlayerWhoInitiated :type Text))
  (LocalVariables|SetLocalMemberID MemberID)
  (LocalVariables|SetLocalTribeID TribeID)
  (LocalVariables|SetLocalPlayerName PlayerWhoInitiated)
  (if (.ReturnValue (Utilities|Map|Find (Variables|Default|GetTribeMap) (LocalVariables|GetLocalTribeID)))
    (LocalVariables|SetLocalMembers (Utilities|Struct|BreakS_TribeInfo (.Value (Utilities|Map|Find (Variables|Default|GetTribeMap) (LocalVariables|GetLocalTribeID)))))
    (bind (_array_element _array_index) (Utilities|Array|ForEachLoopwithBreak (LocalVariables|GetLocalMembers) :!label _label)
      (:LoopBody
        (if (Utilities|Enum|Equal(Enum) (.PlayerIdOffline (Utilities|Struct|BreakS_TribeMemberInfo _array_element)) (LocalVariables|GetLocalMemberID))
          (LocalVariables|SetLocalIndex _array_index)
          (LocalVariables|SetLocalFound? true)
          (goto _label Break)))
      (:Completed
        (if (LocalVariables|GetLocalFound?)
          (bind _structout (Utilities|Struct|SetmembersinS_TribeMemberInfo (Utilities|Array|Get(acopy) (LocalVariables|GetLocalMembers) (LocalVariables|GetLocalIndex)) "NewEnumerator1"))
          (bind _output_get (LocalVariables|SetLocalMemberInfo _structout))
          (Utilities|Array|SetArrayElem (LocalVariables|GetLocalMembers) (LocalVariables|GetLocalIndex) _output_get)
          (bind _structout_2 (Utilities|Struct|SetmembersinS_TribeInfo (.Value (Utilities|Map|Find (Variables|Default|GetTribeMap) (LocalVariables|GetLocalTribeID))) (LocalVariables|GetLocalMembers)))
          (|SetBy-RefVar (Variables|Default|GetTribeMap) (Utilities|Map|MakeMap (LocalVariables|GetLocalTribeID) _structout_2))
          (Utilities|IsValid (.ControllerRef (Utilities|Struct|BreakS_TribeMemberInfo (LocalVariables|GetLocalMemberInfo)))
            (:Is%20Valid
              (Default|UpdateTribeRank (.ControllerRef (Utilities|Struct|BreakS_TribeMemberInfo (LocalVariables|GetLocalMemberInfo))) (.TribeRank (Utilities|Struct|BreakS_TribeMemberInfo (LocalVariables|GetLocalMemberInfo)))))
            (:Is%20Not%20Valid
              _))
          (LocalVariables|SetTribeLogEvent (Utilities|Struct|MakeS_TribeLogEntry (Utilities|Text|ToText(Float) (Actor|GetGameTimeSinceCreation) "HalfToEven") "1" (Utilities|Text|FormatText "{Initiator} Promoted {player} to {Rank}!" (LocalVariables|GetLocalPlayerName) (.PlayerName (Utilities|Struct|BreakS_TribeMemberInfo (LocalVariables|GetLocalMemberInfo))) (Utilities|Text|ToText(String) (Utilities|String|ToString(Byte) (.TribeRank (Utilities|Struct|BreakS_TribeMemberInfo (LocalVariables|GetLocalMemberInfo)))))) "NewEnumerator2"))
          (CallFunction|UpdateMembersandLog (LocalVariables|GetLocalMembers) (LocalVariables|GetTribeLogEvent) (LocalVariables|GetLocalTribeID) true))))))

(fn KickTribeMemberFunction
  (params (PlayerID :type String) (TribeID :type String) (PlayerWhoInitiated :type Text))
  (CallFunction|LeaveTribeFunction PlayerID TribeID true PlayerWhoInitiated))

(fn LeaveTribeFunction
  (params (PlayerID :type String) (TribeID :type String) (KickedOrLeft? :type Boolean) (PlayerWhoInitiated :type Text))
  (LocalVariables|SetLocalPlayerID PlayerID)
  (LocalVariables|SetLocalTribeID TribeID)
  (LocalVariables|SetKickedOrLeftTribe? KickedOrLeft?)
  (LocalVariables|SetLocalPlayerWhoInitiated PlayerWhoInitiated)
  (if (.ReturnValue (Utilities|Map|Find (Variables|Default|GetTribeMap) (LocalVariables|GetLocalTribeID)))
    (LocalVariables|SetLocalMembers (Utilities|Struct|BreakS_TribeInfo (.Value (Utilities|Map|Find (Variables|Default|GetTribeMap) (LocalVariables|GetLocalTribeID)))))
    (bind (_array_element _array_index) (Utilities|Array|ForEachLoopwithBreak (LocalVariables|GetLocalMembers) :!label _label)
      (:LoopBody
        (if (Utilities|Enum|Equal(Enum) (.PlayerIdOffline (Utilities|Struct|BreakS_TribeMemberInfo _array_element)) (LocalVariables|GetLocalPlayerID))
          (if (Utilities|Enum|NotEqual(Enum) (.TribeRank (Utilities|Struct|BreakS_TribeMemberInfo _array_element)) "NewEnumerator0")
            (LocalVariables|SetLocalIndex _array_index)
            (LocalVariables|SetFound? true)
            (goto _label Break))))
      (:Completed
        (if (LocalVariables|GetFound?)
          (LocalVariables|SetLocalPlayerName (.PlayerName (Utilities|Struct|BreakS_TribeMemberInfo (Utilities|Array|Get(acopy) (LocalVariables|GetLocalMembers) (LocalVariables|GetLocalIndex)))))
          (Utilities|IsValid (.ControllerRef (Utilities|Struct|BreakS_TribeMemberInfo (Utilities|Array|Get(acopy) (LocalVariables|GetLocalMembers) (LocalVariables|GetLocalIndex))))
            (:Is%20Valid
              (Default|RemovefromTribe (.ControllerRef (Utilities|Struct|BreakS_TribeMemberInfo (Utilities|Array|Get(acopy) (LocalVariables|GetLocalMembers) (LocalVariables|GetLocalIndex))))))
            (:Is%20Not%20Valid
              _))
          (Utilities|Array|RemoveIndex (LocalVariables|GetLocalMembers) (LocalVariables|GetLocalIndex))
          (bind _structout (Utilities|Struct|SetmembersinS_TribeInfo (.Value (Utilities|Map|Find (Variables|Default|GetTribeMap) (LocalVariables|GetLocalTribeID))) (LocalVariables|GetLocalMembers)))
          (|SetBy-RefVar (Variables|Default|GetTribeMap) (Utilities|Map|MakeMap (LocalVariables|GetLocalTribeID) _structout))
          (LocalVariables|SetTribeLogInfo (Utilities|Struct|MakeS_TribeLogEntry (Utilities|Text|ToText(Float) (Actor|GetGameTimeSinceCreation) "HalfToEven") "1" (select (LocalVariables|GetKickedOrLeftTribe?) (Utilities|Text|FormatText "{initiator} has kicked {player} from the tribe!" (LocalVariables|GetLocalPlayerWhoInitiated) (LocalVariables|GetLocalPlayerName)) (Utilities|Text|FormatText "{player} has left the tribe!" (LocalVariables|GetLocalPlayerName))) "NewEnumerator1"))
          (LocalVariables|SetLocalMembers (Utilities|Struct|BreakS_TribeInfo (.Value (Utilities|Map|Find (Variables|Default|GetTribeMap) (LocalVariables|GetLocalTribeID)))))
          (CallFunction|UpdateMembersandLog (LocalVariables|GetLocalMembers) (LocalVariables|GetTribeLogInfo) (LocalVariables|GetLocalTribeID) true))))))

(fn TribeMessageOftheDay
  (params (TribeID :type String) (MOTD :type Text) (PlayerWhoInitiated :type Text))
  (LocalVariables|SetLocalTribeID TribeID)
  (LocalVariables|SetLocalMOTD MOTD)
  (LocalVariables|SetLocalPlayerName PlayerWhoInitiated)
  (if (.ReturnValue (Utilities|Map|Find (Variables|Default|GetTribeMap) (LocalVariables|GetLocalTribeID)))
    (LocalVariables|SetLocalMembersArray (Utilities|Struct|BreakS_TribeInfo (.Value (Utilities|Map|Find (Variables|Default|GetTribeMap) (LocalVariables|GetLocalTribeID)))))
    (bind _structout (Utilities|Struct|SetmembersinS_TribeInfo (.Value (Utilities|Map|Find (Variables|Default|GetTribeMap) (LocalVariables|GetLocalTribeID))) (LocalVariables|GetLocalMOTD)))
    (|SetBy-RefVar (Variables|Default|GetTribeMap) (Utilities|Map|MakeMap (LocalVariables|GetLocalTribeID) _structout))
    (LocalVariables|SetLogEvent (Utilities|Struct|MakeS_TribeLogEntry (Utilities|Text|ToText(Float) (Actor|GetGameTimeSinceCreation) "HalfToEven") "1" (Utilities|Text|FormatText "{player} Updated the Message of the Day!" (LocalVariables|GetLocalPlayerName)) "NewEnumerator2"))
    (CallFunction|AddLogtoArray (LocalVariables|GetLocalTribeID) (LocalVariables|GetLogEvent))
    (for _array_element (LocalVariables|GetLocalMembersArray)
      (if (and (.IsOnline? (Utilities|Struct|BreakS_TribeMemberInfo _array_element)) (Utilities|IsValid (.ControllerRef (Utilities|Struct|BreakS_TribeMemberInfo _array_element))))
        (Default|UpdateTribeMessage (.ControllerRef (Utilities|Struct|BreakS_TribeMemberInfo _array_element)) (LocalVariables|GetLocalMOTD))
        (Default|UpdateTribeLogUI (.ControllerRef (Utilities|Struct|BreakS_TribeMemberInfo _array_element)) (LocalVariables|GetLogEvent))))))

(fn GetGameStateRef
  (return self))

(fn GetTribeInfo
  (params (TribeID :type String))
  (return (.Value (Utilities|Map|Find (Variables|Default|GetTribeMap) TribeID))))